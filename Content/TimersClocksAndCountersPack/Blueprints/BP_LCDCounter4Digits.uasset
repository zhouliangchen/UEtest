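; Four-digit LCD counter prop that counts up or down to a target number, wrapping between 0 and 9999.
; A re-entering Gate and Delay loop steps the count, controlled by auto-start or Start/Stop events, and flags when the target is reached.
; Each digit is isolated with integer math and shown by swapping static meshes.
; The construction script previews the initial number and configures housing, glass and glow through dynamic material instances.
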(event `self.ReceiveBeginPlay`
  (bind _currentnumber (`self.CurrentNumber`))
  (bind _returnvalue (!= (`self.TargetNumber`) (`self.CurrentNumber`)))
  ;[1 1 1] Set funtion of counter
  (set `self.CurrentNumber` (`self.InitialNumber`))
  (`/Engine/EditorBlueprintResources/StandardMacros.Gate` (not (`self.AutoStartCounter`)) :!label _label
    (:`Exit`
      (switch `/Game/TimersClocksAndCountersPack/Enum_CounterFunction` (`self.CounterFunction`)
        (:`NewEnumerator1`
          (if _returnvalue
            (`KismetSystemLibrary.Delay` (`self.CounterDelayTime`))
            (`/Engine/EditorBlueprintResources/StandardMacros.IncrementInt` _currentnumber
              (:`  `
                (if (> _currentnumber 9999)
                  (set `self.CurrentNumber` 0))
                (`self.EventUpdateDisplay` :!label _label_2)
                (goto _label)))
            (else
              _)))
        (:`NewEnumerator2`
          (if _returnvalue
            (`KismetSystemLibrary.Delay` (`self.CounterDelayTime`))
            (`/Engine/EditorBlueprintResources/StandardMacros.DecrementInt` _currentnumber
              (:`  `
                (if (< _currentnumber 0)
                  (set `self.CurrentNumber` 9999)
                  (goto _label_2)
                  (else
                    (goto _label_2)))))
            (else
              _))))
      (`self.EventTargetNumberReached`))))

(event `StartTimer`
  ;[1 1 1] Call the Start Timer or Stop Timer Events to start/stop the timer during gameplay
  (`|ExecutionSequence`
    (:`then_0`
      (goto _label :!via `Open`))
    (:`then_1`
      (goto _label))))

(event `StopTimer`
  ;[1 1 1] Call the Start Timer or Stop Timer Events to start/stop the timer during gameplay
  (goto _label :!via `Close`))

(event `EventResetCounter`
  ;[1 1 1] Call this event to reset the counter to it's initial value.(Call EventStartTimer to start the timer again.)
  (set `self.CurrentNumber` (`self.InitialNumber`))
  (set `self.IsAtTarget` false))

(event `EventUpdateDisplay`
  (bind _currentnumber (`self.CurrentNumber`))
  (bind _returnvalue (/ _currentnumber 1000))
  (bind _returnvalue_2 (- (/ _currentnumber 100) (* _returnvalue 10)))
  (bind _returnvalue_3 (- (- (/ _currentnumber 10) (* _returnvalue 100)) (* _returnvalue_2 10)))
  ;[1 1 1] Updates the display to display the value of "CurrentNumber"
  (`StaticMeshComponent.SetStaticMesh` (`self.Thousands`) (select `int` _returnvalue :`0` "/Game/TimersClocksAndCountersPack/Meshes/SM_LCD0.SM_LCD0" :`1` "/Game/TimersClocksAndCountersPack/Meshes/SM_LCD1.SM_LCD1" :`2` "/Game/TimersClocksAndCountersPack/Meshes/SM_LCD2.SM_LCD2" :`3` "/Game/TimersClocksAndCountersPack/Meshes/SM_LCD3.SM_LCD3" :`4` "/Game/TimersClocksAndCountersPack/Meshes/SM_LCD4.SM_LCD4" :`5` "/Game/TimersClocksAndCountersPack/Meshes/SM_LCD5.SM_LCD5" :`6` "/Game/TimersClocksAndCountersPack/Meshes/SM_LCD6.SM_LCD6" :`7` "/Game/TimersClocksAndCountersPack/Meshes/SM_LCD7.SM_LCD7" :`8` "/Game/TimersClocksAndCountersPack/Meshes/SM_LCD8.SM_LCD8" :`9` "/Game/TimersClocksAndCountersPack/Meshes/SM_LCD9.SM_LCD9" :!type "StaticMesh Object Reference"))
  (`StaticMeshComponent.SetStaticMesh` (`self.Hundreds`) (select `int` _returnvalue_2 :`0` "/Game/TimersClocksAndCountersPack/Meshes/SM_LCD0.SM_LCD0" :`1` "/Game/TimersClocksAndCountersPack/Meshes/SM_LCD1.SM_LCD1" :`2` "/Game/TimersClocksAndCountersPack/Meshes/SM_LCD2.SM_LCD2" :`3` "/Game/TimersClocksAndCountersPack/Meshes/SM_LCD3.SM_LCD3" :`4` "/Game/TimersClocksAndCountersPack/Meshes/SM_LCD4.SM_LCD4" :`5` "/Game/TimersClocksAndCountersPack/Meshes/SM_LCD5.SM_LCD5" :`6` "/Game/TimersClocksAndCountersPack/Meshes/SM_LCD6.SM_LCD6" :`7` "/Game/TimersClocksAndCountersPack/Meshes/SM_LCD7.SM_LCD7" :`8` "/Game/TimersClocksAndCountersPack/Meshes/SM_LCD8.SM_LCD8" :`9` "/Game/TimersClocksAndCountersPack/Meshes/SM_LCD9.SM_LCD9" :!type "StaticMesh Object Reference"))
  (`StaticMeshComponent.SetStaticMesh` (`self.Tens`) (select `int` _returnvalue_3 :`0` "/Game/TimersClocksAndCountersPack/Meshes/SM_LCD0.SM_LCD0" :`1` "/Game/TimersClocksAndCountersPack/Meshes/SM_LCD1.SM_LCD1" :`2` "/Game/TimersClocksAndCountersPack/Meshes/SM_LCD2.SM_LCD2" :`3` "/Game/TimersClocksAndCountersPack/Meshes/SM_LCD3.SM_LCD3" :`4` "/Game/TimersClocksAndCountersPack/Meshes/SM_LCD4.SM_LCD4" :`5` "/Game/TimersClocksAndCountersPack/Meshes/SM_LCD5.SM_LCD5" :`6` "/Game/TimersClocksAndCountersPack/Meshes/SM_LCD6.SM_LCD6" :`7` "/Game/TimersClocksAndCountersPack/Meshes/SM_LCD7.SM_LCD7" :`8` "/Game/TimersClocksAndCountersPack/Meshes/SM_LCD8.SM_LCD8" :`9` "/Game/TimersClocksAndCountersPack/Meshes/SM_LCD9.SM_LCD9" :!type "StaticMesh Object Reference"))
  (`StaticMeshComponent.SetStaticMesh` (`self.Ones`) (select `int` (- (- (- _currentnumber (* _returnvalue 1000)) (* _returnvalue_2 100)) (* _returnvalue_3 10)) :`0` "/Game/TimersClocksAndCountersPack/Meshes/SM_LCD0.SM_LCD0" :`1` "/Game/TimersClocksAndCountersPack/Meshes/SM_LCD1.SM_LCD1" :`2` "/Game/TimersClocksAndCountersPack/Meshes/SM_LCD2.SM_LCD2" :`3` "/Game/TimersClocksAndCountersPack/Meshes/SM_LCD3.SM_LCD3" :`4` "/Game/TimersClocksAndCountersPack/Meshes/SM_LCD4.SM_LCD4" :`5` "/Game/TimersClocksAndCountersPack/Meshes/SM_LCD5.SM_LCD5" :`6` "/Game/TimersClocksAndCountersPack/Meshes/SM_LCD6.SM_LCD6" :`7` "/Game/TimersClocksAndCountersPack/Meshes/SM_LCD7.SM_LCD7" :`8` "/Game/TimersClocksAndCountersPack/Meshes/SM_LCD8.SM_LCD8" :`9` "/Game/TimersClocksAndCountersPack/Meshes/SM_LCD9.SM_LCD9" :!type "StaticMesh Object Reference")))

(event `EventTargetNumberReached`
  ;[1 1 1] This Event will be triggered when the target number is reached
  (set `self.IsAtTarget` true))

(fn `UserConstructionScript`
  (bind _housingvariation (`self.HousingVariation`))
  (bind _housingmesh (`self.HousingMesh`))
  (bind _initialnumber (`self.InitialNumber`))
  (bind _returnvalue (!= _housingvariation 0))
  (bind _returnvalue_2 (/ _initialnumber 1000))
  (bind _returnvalue_3 (- (/ _initialnumber 100) (* _returnvalue_2 10)))
  (bind _returnvalue_4 (- (- (/ _initialnumber 10) (* _returnvalue_2 100)) (* _returnvalue_3 10)))
  ;[1 1 1] Get System time and apply correct values to all displays
  (`StaticMeshComponent.SetStaticMesh` (`self.Thousands`) (select `int` _returnvalue_2 :`0` "/Game/TimersClocksAndCountersPack/Meshes/SM_LCD0.SM_LCD0" :`1` "/Game/TimersClocksAndCountersPack/Meshes/SM_LCD1.SM_LCD1" :`2` "/Game/TimersClocksAndCountersPack/Meshes/SM_LCD2.SM_LCD2" :`3` "/Game/TimersClocksAndCountersPack/Meshes/SM_LCD3.SM_LCD3" :`4` "/Game/TimersClocksAndCountersPack/Meshes/SM_LCD4.SM_LCD4" :`5` "/Game/TimersClocksAndCountersPack/Meshes/SM_LCD5.SM_LCD5" :`6` "/Game/TimersClocksAndCountersPack/Meshes/SM_LCD6.SM_LCD6" :`7` "/Game/TimersClocksAndCountersPack/Meshes/SM_LCD7.SM_LCD7" :`8` "/Game/TimersClocksAndCountersPack/Meshes/SM_LCD8.SM_LCD8" :`9` "/Game/TimersClocksAndCountersPack/Meshes/SM_LCD9.SM_LCD9" :!type "StaticMesh Object Reference"))
  (`StaticMeshComponent.SetStaticMesh` (`self.Hundreds`) (select `int` _returnvalue_3 :`0` "/Game/TimersClocksAndCountersPack/Meshes/SM_LCD0.SM_LCD0" :`1` "/Game/TimersClocksAndCountersPack/Meshes/SM_LCD1.SM_LCD1" :`2` "/Game/TimersClocksAndCountersPack/Meshes/SM_LCD2.SM_LCD2" :`3` "/Game/TimersClocksAndCountersPack/Meshes/SM_LCD3.SM_LCD3" :`4` "/Game/TimersClocksAndCountersPack/Meshes/SM_LCD4.SM_LCD4" :`5` "/Game/TimersClocksAndCountersPack/Meshes/SM_LCD5.SM_LCD5" :`6` "/Game/TimersClocksAndCountersPack/Meshes/SM_LCD6.SM_LCD6" :`7` "/Game/TimersClocksAndCountersPack/Meshes/SM_LCD7.SM_LCD7" :`8` "/Game/TimersClocksAndCountersPack/Meshes/SM_LCD8.SM_LCD8" :`9` "/Game/TimersClocksAndCountersPack/Meshes/SM_LCD9.SM_LCD9" :!type "StaticMesh Object Reference"))
  (`StaticMeshComponent.SetStaticMesh` (`self.Tens`) (select `int` _returnvalue_4 :`0` "/Game/TimersClocksAndCountersPack/Meshes/SM_LCD0.SM_LCD0" :`1` "/Game/TimersClocksAndCountersPack/Meshes/SM_LCD1.SM_LCD1" :`2` "/Game/TimersClocksAndCountersPack/Meshes/SM_LCD2.SM_LCD2" :`3` "/Game/TimersClocksAndCountersPack/Meshes/SM_LCD3.SM_LCD3" :`4` "/Game/TimersClocksAndCountersPack/Meshes/SM_LCD4.SM_LCD4" :`5` "/Game/TimersClocksAndCountersPack/Meshes/SM_LCD5.SM_LCD5" :`6` "/Game/TimersClocksAndCountersPack/Meshes/SM_LCD6.SM_LCD6" :`7` "/Game/TimersClocksAndCountersPack/Meshes/SM_LCD7.SM_LCD7" :`8` "/Game/TimersClocksAndCountersPack/Meshes/SM_LCD8.SM_LCD8" :`9` "/Game/TimersClocksAndCountersPack/Meshes/SM_LCD9.SM_LCD9" :!type "StaticMesh Object Reference"))
  (`StaticMeshComponent.SetStaticMesh` (`self.Ones`) (select `int` (- (- (- _initialnumber (* _returnvalue_2 1000)) (* _returnvalue_3 100)) (* _returnvalue_4 10)) :`0` "/Game/TimersClocksAndCountersPack/Meshes/SM_LCD0.SM_LCD0" :`1` "/Game/TimersClocksAndCountersPack/Meshes/SM_LCD1.SM_LCD1" :`2` "/Game/TimersClocksAndCountersPack/Meshes/SM_LCD2.SM_LCD2" :`3` "/Game/TimersClocksAndCountersPack/Meshes/SM_LCD3.SM_LCD3" :`4` "/Game/TimersClocksAndCountersPack/Meshes/SM_LCD4.SM_LCD4" :`5` "/Game/TimersClocksAndCountersPack/Meshes/SM_LCD5.SM_LCD5" :`6` "/Game/TimersClocksAndCountersPack/Meshes/SM_LCD6.SM_LCD6" :`7` "/Game/TimersClocksAndCountersPack/Meshes/SM_LCD7.SM_LCD7" :`8` "/Game/TimersClocksAndCountersPack/Meshes/SM_LCD8.SM_LCD8" :`9` "/Game/TimersClocksAndCountersPack/Meshes/SM_LCD9.SM_LCD9" :!type "StaticMesh Object Reference"))
  ;[1 1 1] Apply setting as set by the user
  (`SceneComponent.SetVisibility` _housingmesh _returnvalue false)
  (`PrimitiveComponent.SetCastShadow` _housingmesh _returnvalue)
  (`StaticMeshComponent.SetStaticMesh` _housingmesh (select `int` _housingvariation :`0` "/Game/TimersClocksAndCountersPack/Meshes/SM_LCDHousing03.SM_LCDHousing03" :`1` "/Game/TimersClocksAndCountersPack/Meshes/SM_LCDHousing03.SM_LCDHousing03" :`2` "/Game/TimersClocksAndCountersPack/Meshes/SM_LCDHousing02.SM_LCDHousing02" :!type "StaticMesh Object Reference"))
  (bind _returnvalue_5 (`KismetMaterialLibrary.CreateDynamicMaterialInstance` "/Game/TimersClocksAndCountersPack/Materials/M_LCDNumbers_Inst.M_LCDNumbers_Inst"))
  (bind _output_get (set `self.DynMatLCD` _returnvalue_5))
  (`PrimitiveComponent.SetMaterial` (`self.Ones`) 0 _output_get)
  (`PrimitiveComponent.SetMaterial` (`self.Tens`) 0 _output_get)
  (`PrimitiveComponent.SetMaterial` (`self.Hundreds`) 0 _output_get)
  (`PrimitiveComponent.SetMaterial` (`self.Thousands`) 0 _output_get)
  (`MaterialInstanceDynamic.SetScalarParameterValue` _output_get "EmissiveMultiplier" (`self.DisplayGlowBrightness`))
  (`MaterialInstanceDynamic.SetVectorParameterValue` _output_get "GlowColor" (`self.DisplayGlowColor`))
  (bind _returnvalue_6 (`KismetMaterialLibrary.CreateDynamicMaterialInstance` "/Game/TimersClocksAndCountersPack/Materials/M_LCDGlass_Inst.M_LCDGlass_Inst"))
  (bind _output_get_2 (set `self.DynMatGlass` _returnvalue_6))
  (`PrimitiveComponent.SetMaterial` (`self.HousingMesh`) 1 _output_get_2)
  (`MaterialInstanceDynamic.SetScalarParameterValue` _output_get_2 "OpacityMultiplier" (`self.OpacityGlass`))
  (`MaterialInstanceDynamic.SetScalarParameterValue` _output_get_2 "New-Old" (`self.AgeGlass`))
  (`MaterialInstanceDynamic.SetScalarParameterValue` _output_get_2 "Roughness" (`self.RoughnessGlass`))
  (`MaterialInstanceDynamic.SetScalarParameterValue` _output_get_2 "NormalMapStrength" (`self.NormalMapStrengthGlass`))
  (bind _returnvalue_7 (`KismetMaterialLibrary.CreateDynamicMaterialInstance` (select `/Game/TimersClocksAndCountersPack/Enum_Material` (`self.HousingMaterial`) :`NewEnumerator0` "/Game/TimersClocksAndCountersPack/Materials/M_LCDHousing2_Inst.M_LCDHousing2_Inst" :`NewEnumerator1` "/Game/TimersClocksAndCountersPack/Materials/M_LCDHousing1_Inst.M_LCDHousing1_Inst" :!type "MaterialInterface Object Reference")))
  (bind _output_get_3 (set `self.DynMatHousing` _returnvalue_7))
  (`PrimitiveComponent.SetMaterial` (`self.HousingMesh`) 0 _output_get_3)
  (`MaterialInstanceDynamic.SetScalarParameterValue` _output_get_3 "New-Old" (`self.AgeHousing`))
  (`MaterialInstanceDynamic.SetScalarParameterValue` _output_get_3 "FadeOutTexture" (`self.FadeOutTextureHousing`))
  (`MaterialInstanceDynamic.SetScalarParameterValue` _output_get_3 "DesaturateTexture" (`self.DesaturateTextureHousing`))
  (`MaterialInstanceDynamic.SetScalarParameterValue` _output_get_3 "Metallic" (`self.MetallicHousing`))
  (`MaterialInstanceDynamic.SetScalarParameterValue` _output_get_3 "Roughness" (`self.RoughnessHousing`))
  (`MaterialInstanceDynamic.SetScalarParameterValue` _output_get_3 "Specular" (`self.SpecularHousing`))
  (`MaterialInstanceDynamic.SetScalarParameterValue` _output_get_3 "NormalMapStrength" (`self.NormalMapStrengthHousing`))
  (`MaterialInstanceDynamic.SetVectorParameterValue` _output_get_3 "Tint" (`self.TintHousing`)))