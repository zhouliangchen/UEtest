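; Nixie-style valve tube display that glows one digit from 0 to 9, or a colon, using a separate plate mesh for each symbol.
; The construction script handles flipping, randomizes yaw, creates dynamic materials and lights the initial symbol in GlowColor.
; EventApplyValue relights the plate matching DisplayNumber by swapping opacity textures and emissive brightness, scaled per digit.
; An unconnected once-per-second digit-cycling loop never runs.
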(event `self.ReceiveBeginPlay`)

(event `EventApplyValue`
  (bind _dynmatplate0 (`self.DynMatPlate0`))
  (bind _displaynumber (`self.DisplayNumber`))
  (bind _returnvalue (select `int` _displaynumber :`0` _dynmatplate0 :`1` (`self.DynMatPlate1`) :`2` (`self.DynMatPlate2`) :`3` (`self.DynMatPlate3`) :`4` (`self.DynMatPlate4`) :`5` (`self.DynMatPlate5`) :`6` (`self.DynMatPlate6`) :`7` (`self.DynMatPlate7`) :`8` (`self.DynMatPlate8`) :`9` (`self.DynMatPlate9`)))
  (`MaterialInstanceDynamic.SetScalarParameterValue` _dynmatplate0 "EmissiveBrightness" 0.0)
  (`MaterialInstanceDynamic.SetScalarParameterValue` (`self.DynMatPlate1`) "EmissiveBrightness" 0.0)
  (`MaterialInstanceDynamic.SetScalarParameterValue` (`self.DynMatPlate2`) "EmissiveBrightness" 0.0)
  (`MaterialInstanceDynamic.SetScalarParameterValue` (`self.DynMatPlate3`) "EmissiveBrightness" 0.0)
  (`MaterialInstanceDynamic.SetScalarParameterValue` (`self.DynMatPlate9`) "EmissiveBrightness" 0.0)
  (`MaterialInstanceDynamic.SetScalarParameterValue` (`self.DynMatPlate8`) "EmissiveBrightness" 0.0)
  (`MaterialInstanceDynamic.SetScalarParameterValue` (`self.DynMatPlate6`) "EmissiveBrightness" 0.0)
  (`MaterialInstanceDynamic.SetScalarParameterValue` (`self.DynMatPlate7`) "EmissiveBrightness" 0.0)
  (`MaterialInstanceDynamic.SetScalarParameterValue` (`self.DynMatPlate5`) "EmissiveBrightness" 0.0)
  (`MaterialInstanceDynamic.SetScalarParameterValue` (`self.DynMatPlate4`) "EmissiveBrightness" 0.0)
  (`MaterialInstanceDynamic.SetTextureParameterValue` _dynmatplate0 "OpacityTexture" "/Game/TimersClocksAndCountersPack/Textures/O_DialsAndCounters01Off.O_DialsAndCounters01Off")
  (`MaterialInstanceDynamic.SetTextureParameterValue` (`self.DynMatPlate1`) "OpacityTexture" "/Game/TimersClocksAndCountersPack/Textures/O_DialsAndCounters01Off.O_DialsAndCounters01Off")
  (`MaterialInstanceDynamic.SetTextureParameterValue` (`self.DynMatPlate2`) "OpacityTexture" "/Game/TimersClocksAndCountersPack/Textures/O_DialsAndCounters01Off.O_DialsAndCounters01Off")
  (`MaterialInstanceDynamic.SetTextureParameterValue` (`self.DynMatPlate3`) "OpacityTexture" "/Game/TimersClocksAndCountersPack/Textures/O_DialsAndCounters01Off.O_DialsAndCounters01Off")
  (`MaterialInstanceDynamic.SetTextureParameterValue` (`self.DynMatPlate4`) "OpacityTexture" "/Game/TimersClocksAndCountersPack/Textures/O_DialsAndCounters01Off.O_DialsAndCounters01Off")
  (`MaterialInstanceDynamic.SetTextureParameterValue` (`self.DynMatPlate5`) "OpacityTexture" "/Game/TimersClocksAndCountersPack/Textures/O_DialsAndCounters01Off.O_DialsAndCounters01Off")
  (`MaterialInstanceDynamic.SetTextureParameterValue` (`self.DynMatPlate6`) "OpacityTexture" "/Game/TimersClocksAndCountersPack/Textures/O_DialsAndCounters01Off.O_DialsAndCounters01Off")
  (`MaterialInstanceDynamic.SetTextureParameterValue` (`self.DynMatPlate7`) "OpacityTexture" "/Game/TimersClocksAndCountersPack/Textures/O_DialsAndCounters01Off.O_DialsAndCounters01Off")
  (`MaterialInstanceDynamic.SetTextureParameterValue` (`self.DynMatPlate8`) "OpacityTexture" "/Game/TimersClocksAndCountersPack/Textures/O_DialsAndCounters01Off.O_DialsAndCounters01Off")
  (`MaterialInstanceDynamic.SetTextureParameterValue` (`self.DynMatPlate9`) "OpacityTexture" "/Game/TimersClocksAndCountersPack/Textures/O_DialsAndCounters01Off.O_DialsAndCounters01Off")
  (`MaterialInstanceDynamic.SetScalarParameterValue` _returnvalue "EmissiveBrightness" (* (`self.GlowBrightness`) (select `int` _displaynumber :`0` 11.0 :`1` 1.0 :`2` 1.0 :`3` 1.0 :`4` 1.3 :`5` 2.0 :`6` 3.0 :`7` 5.0 :`8` 7.0 :`9` 8.0 :!type "Float (single-precision)")))
  (`MaterialInstanceDynamic.SetTextureParameterValue` _returnvalue "OpacityTexture" "/Game/TimersClocksAndCountersPack/Textures/O_DialsAndCounters01On.O_DialsAndCounters01On"))

(fn `UserConstructionScript`
  (bind _dynmatplate0 (`self.DynMatPlate0`))
  (bind _displaynumber (`self.DisplayNumber`))
  (bind _dynmatplatecolon (`self.DynMatPlateColon`))
  (bind _flipupdirection (`self.FlipUpDirection`))
  (bind _returnvalue (select `int` _displaynumber :`0` _dynmatplate0 :`1` (`self.DynMatPlate1`) :`2` (`self.DynMatPlate2`) :`3` (`self.DynMatPlate3`) :`4` (`self.DynMatPlate4`) :`5` (`self.DynMatPlate5`) :`6` (`self.DynMatPlate6`) :`7` (`self.DynMatPlate7`) :`8` (`self.DynMatPlate8`) :`9` (`self.DynMatPlate9`)))
  (bind _returnvalue_2 (select `bool` _flipupdirection :`true` (struct :`Pitch` 180.0) :!type "Rotator Structure"))
  (bind _pitch (.pitch _returnvalue_2))
  ;[1 1 1] Set Up-direction
  (`SceneComponent.K2_SetRelativeRotation` (`self.CounterMesh0`) _returnvalue_2 false false)
  (`SceneComponent.K2_SetRelativeRotation` (`self.CounterMesh1`) _returnvalue_2 false false)
  (`SceneComponent.K2_SetRelativeRotation` (`self.CounterMesh2`) _returnvalue_2 false false)
  (`SceneComponent.K2_SetRelativeRotation` (`self.CounterMesh3`) _returnvalue_2 false false)
  (`SceneComponent.K2_SetRelativeRotation` (`self.CounterMesh4`) _returnvalue_2 false false)
  (`SceneComponent.K2_SetRelativeRotation` (`self.CounterMesh5`) _returnvalue_2 false false)
  (`SceneComponent.K2_SetRelativeRotation` (`self.CounterMesh6`) _returnvalue_2 false false)
  (`SceneComponent.K2_SetRelativeRotation` (`self.CounterMesh7`) _returnvalue_2 false false)
  (`SceneComponent.K2_SetRelativeRotation` (`self.CounterMesh8`) _returnvalue_2 false false)
  (`SceneComponent.K2_SetRelativeRotation` (`self.CounterMesh9`) _returnvalue_2 false false)
  (`SceneComponent.K2_SetRelativeRotation` (`self.SM_Valve`) _returnvalue_2 false false)
  (`SceneComponent.K2_SetRelativeRotation` (`self.CounterMeshColon`) _returnvalue_2 false false)
  (`SceneComponent.K2_SetRelativeLocation` (`self.CounterMesh0`) (select `bool` _flipupdirection :`false` (0.0 0.0 0.5) :`true` (0.0 0.0 9.1) :!type "Vector Structure") false false)
  (`SceneComponent.K2_SetRelativeLocation` (`self.CounterMesh1`) (select `bool` _flipupdirection :`false` (0.0 0.0 0.5) :`true` (0.0 0.0 9.1) :!type "Vector Structure") false false)
  (`SceneComponent.K2_SetRelativeLocation` (`self.CounterMesh2`) (select `bool` _flipupdirection :`false` (0.0 0.0 0.5) :`true` (0.0 0.0 9.1) :!type "Vector Structure") false false)
  (`SceneComponent.K2_SetRelativeLocation` (`self.CounterMesh3`) (select `bool` _flipupdirection :`false` (0.0 0.0 0.5) :`true` (0.0 0.0 9.1) :!type "Vector Structure") false false)
  (`SceneComponent.K2_SetRelativeLocation` (`self.CounterMesh4`) (select `bool` _flipupdirection :`false` (0.0 0.0 0.5) :`true` (0.0 0.0 9.1) :!type "Vector Structure") false false)
  (`SceneComponent.K2_SetRelativeLocation` (`self.CounterMesh5`) (select `bool` _flipupdirection :`false` (0.0 0.0 0.5) :`true` (0.0 0.0 9.1) :!type "Vector Structure") false false)
  (`SceneComponent.K2_SetRelativeLocation` (`self.CounterMesh6`) (select `bool` _flipupdirection :`false` (0.0 0.0 0.5) :`true` (0.0 0.0 9.1) :!type "Vector Structure") false false)
  (`SceneComponent.K2_SetRelativeLocation` (`self.CounterMesh7`) (select `bool` _flipupdirection :`false` (0.0 0.0 0.5) :`true` (0.0 0.0 9.1) :!type "Vector Structure") false false)
  (`SceneComponent.K2_SetRelativeLocation` (`self.CounterMesh8`) (select `bool` _flipupdirection :`false` (0.0 0.0 0.5) :`true` (0.0 0.0 9.1) :!type "Vector Structure") false false)
  (`SceneComponent.K2_SetRelativeLocation` (`self.CounterMesh9`) (select `bool` _flipupdirection :`false` (0.0 0.0 0.5) :`true` (0.0 0.0 9.1) :!type "Vector Structure") false false)
  (`SceneComponent.K2_SetRelativeLocation` (`self.CounterMeshColon`) (select `bool` _flipupdirection :`false` (0.0 0.0 0.5) :`true` (0.0 0.0 9.1) :!type "Vector Structure") false false)
  (bind _output_get (set `self.RandomRotation` (`KismetMathLibrary.RandomFloatInRange` 0.0 360.0)))
  (`SceneComponent.K2_SetRelativeRotation` (`self.SM_Valve`) (`KismetMathLibrary.MakeRotator` 0.0 _pitch _output_get) false false)
  (`SceneComponent.K2_SetRelativeRotation` (`self.CounterMesh9`) (`KismetMathLibrary.MakeRotator` 0.0 _pitch (* _output_get (select `bool` _flipupdirection :`false` -1.0 :`true` 1.0 :!type "Float (single-precision)"))) false false)
  (`SceneComponent.K2_SetRelativeRotation` (`self.CounterMesh8`) (`KismetMathLibrary.MakeRotator` 0.0 _pitch (* _output_get (select `bool` _flipupdirection :`false` -1.0 :`true` 1.0 :!type "Float (single-precision)"))) false false)
  (`SceneComponent.K2_SetRelativeRotation` (`self.CounterMesh7`) (`KismetMathLibrary.MakeRotator` 0.0 _pitch (* _output_get (select `bool` _flipupdirection :`false` -1.0 :`true` 1.0 :!type "Float (single-precision)"))) false false)
  (`SceneComponent.K2_SetRelativeRotation` (`self.CounterMesh6`) (`KismetMathLibrary.MakeRotator` 0.0 _pitch (* _output_get (select `bool` _flipupdirection :`false` -1.0 :`true` 1.0 :!type "Float (single-precision)"))) false false)
  (`SceneComponent.K2_SetRelativeRotation` (`self.CounterMesh5`) (`KismetMathLibrary.MakeRotator` 0.0 _pitch (* _output_get (select `bool` _flipupdirection :`false` -1.0 :`true` 1.0 :!type "Float (single-precision)"))) false false)
  (`SceneComponent.K2_SetRelativeRotation` (`self.CounterMeshColon`) (`KismetMathLibrary.MakeRotator` 0.0 _pitch (* _output_get (select `bool` _flipupdirection :`false` -1.0 :`true` 1.0 :!type "Float (single-precision)"))) false false)
  (`SceneComponent.K2_SetRelativeRotation` (`self.CounterMesh3`) (`KismetMathLibrary.MakeRotator` 0.0 _pitch (* _output_get (select `bool` _flipupdirection :`false` -1.0 :`true` 1.0 :!type "Float (single-precision)"))) false false)
  (`SceneComponent.K2_SetRelativeRotation` (`self.CounterMesh2`) (`KismetMathLibrary.MakeRotator` 0.0 _pitch (* _output_get (select `bool` _flipupdirection :`false` -1.0 :`true` 1.0 :!type "Float (single-precision)"))) false false)
  (`SceneComponent.K2_SetRelativeRotation` (`self.CounterMesh1`) (`KismetMathLibrary.MakeRotator` 0.0 _pitch (* _output_get (select `bool` _flipupdirection :`false` -1.0 :`true` 1.0 :!type "Float (single-precision)"))) false false)
  (`SceneComponent.K2_SetRelativeRotation` (`self.CounterMesh0`) (`KismetMathLibrary.MakeRotator` 0.0 _pitch (* _output_get (select `bool` _flipupdirection :`false` -1.0 :`true` 1.0 :!type "Float (single-precision)"))) false false)
  (`SceneComponent.K2_SetRelativeRotation` (`self.CounterMesh4`) (`KismetMathLibrary.MakeRotator` 0.0 _pitch (* _output_get (select `bool` _flipupdirection :`false` -1.0 :`true` 1.0 :!type "Float (single-precision)"))) false false)
  ;[1 1 1] Create and apply Dynamic material instances
  (bind _returnvalue_3 (`KismetMaterialLibrary.CreateDynamicMaterialInstance` "/Game/TimersClocksAndCountersPack/Materials/M_ValveCounterPlates_Inst.M_ValveCounterPlates_Inst"))
  (set `self.DynMatPlate0` _returnvalue_3)
  (bind _returnvalue_4 (`KismetMaterialLibrary.CreateDynamicMaterialInstance` "/Game/TimersClocksAndCountersPack/Materials/M_ValveCounterPlates_Inst.M_ValveCounterPlates_Inst"))
  (set `self.DynMatPlate1` _returnvalue_4)
  (bind _returnvalue_5 (`KismetMaterialLibrary.CreateDynamicMaterialInstance` "/Game/TimersClocksAndCountersPack/Materials/M_ValveCounterPlates_Inst.M_ValveCounterPlates_Inst"))
  (set `self.DynMatPlate2` _returnvalue_5)
  (bind _returnvalue_6 (`KismetMaterialLibrary.CreateDynamicMaterialInstance` "/Game/TimersClocksAndCountersPack/Materials/M_ValveCounterPlates_Inst.M_ValveCounterPlates_Inst"))
  (set `self.DynMatPlate3` _returnvalue_6)
  (bind _returnvalue_7 (`KismetMaterialLibrary.CreateDynamicMaterialInstance` "/Game/TimersClocksAndCountersPack/Materials/M_ValveCounterPlates_Inst.M_ValveCounterPlates_Inst"))
  (set `self.DynMatPlate4` _returnvalue_7)
  (bind _returnvalue_8 (`KismetMaterialLibrary.CreateDynamicMaterialInstance` "/Game/TimersClocksAndCountersPack/Materials/M_ValveCounterPlates_Inst.M_ValveCounterPlates_Inst"))
  (set `self.DynMatPlate5` _returnvalue_8)
  (bind _returnvalue_9 (`KismetMaterialLibrary.CreateDynamicMaterialInstance` "/Game/TimersClocksAndCountersPack/Materials/M_ValveCounterPlates_Inst.M_ValveCounterPlates_Inst"))
  (set `self.DynMatPlate6` _returnvalue_9)
  (bind _returnvalue_10 (`KismetMaterialLibrary.CreateDynamicMaterialInstance` "/Game/TimersClocksAndCountersPack/Materials/M_ValveCounterPlates_Inst.M_ValveCounterPlates_Inst"))
  (set `self.DynMatPlate7` _returnvalue_10)
  (bind _returnvalue_11 (`KismetMaterialLibrary.CreateDynamicMaterialInstance` "/Game/TimersClocksAndCountersPack/Materials/M_ValveCounterPlates_Inst.M_ValveCounterPlates_Inst"))
  (set `self.DynMatPlate8` _returnvalue_11)
  (bind _returnvalue_12 (`KismetMaterialLibrary.CreateDynamicMaterialInstance` "/Game/TimersClocksAndCountersPack/Materials/M_ValveCounterPlates_Inst.M_ValveCounterPlates_Inst"))
  (set `self.DynMatPlate9` _returnvalue_12)
  (bind _returnvalue_13 (`KismetMaterialLibrary.CreateDynamicMaterialInstance` "/Game/TimersClocksAndCountersPack/Materials/M_ValveCounterPlates_Inst.M_ValveCounterPlates_Inst"))
  (set `self.DynMatPlateColon` _returnvalue_13)
  (`PrimitiveComponent.SetMaterial` (`self.CounterMesh0`) 0 (`self.DynMatPlate0`))
  (`PrimitiveComponent.SetMaterial` (`self.CounterMesh1`) 0 (`self.DynMatPlate1`))
  (`PrimitiveComponent.SetMaterial` (`self.CounterMesh2`) 0 (`self.DynMatPlate2`))
  (`PrimitiveComponent.SetMaterial` (`self.CounterMesh3`) 0 (`self.DynMatPlate3`))
  (`PrimitiveComponent.SetMaterial` (`self.CounterMesh4`) 0 (`self.DynMatPlate4`))
  (`PrimitiveComponent.SetMaterial` (`self.CounterMesh5`) 0 (`self.DynMatPlate5`))
  (`PrimitiveComponent.SetMaterial` (`self.CounterMesh6`) 0 (`self.DynMatPlate6`))
  (`PrimitiveComponent.SetMaterial` (`self.CounterMesh7`) 0 (`self.DynMatPlate7`))
  (`PrimitiveComponent.SetMaterial` (`self.CounterMesh8`) 0 (`self.DynMatPlate8`))
  (`PrimitiveComponent.SetMaterial` (`self.CounterMesh9`) 0 (`self.DynMatPlate9`))
  (`PrimitiveComponent.SetMaterial` (`self.CounterMeshColon`) 0 (`self.DynMatPlateColon`))
  (bind _returnvalue_14 (`KismetMaterialLibrary.CreateDynamicMaterialInstance` "/Game/TimersClocksAndCountersPack/Materials/M_ValveEnds_Inst.M_ValveEnds_Inst"))
  (bind _output_get_2 (set `self.DynMatValveEnds` _returnvalue_14))
  (bind _returnvalue_15 (`KismetMaterialLibrary.CreateDynamicMaterialInstance` "/Game/TimersClocksAndCountersPack/Materials/M_ValveGlass_Inst.M_ValveGlass_Inst"))
  (bind _output_get_3 (set `self.DynMatValveGlass` _returnvalue_15))
  (`PrimitiveComponent.SetMaterial` (`self.SM_Valve`) 1 _output_get_3)
  (`PrimitiveComponent.SetMaterial` (`self.SM_Valve`) 0 _output_get_2)
  ;[1 1 1] Apply settings to display the correct number
  (`MaterialInstanceDynamic.SetTextureParameterValue` _dynmatplate0 "OpacityTexture" "/Game/TimersClocksAndCountersPack/Textures/O_DialsAndCounters01Off.O_DialsAndCounters01Off")
  (`MaterialInstanceDynamic.SetTextureParameterValue` (`self.DynMatPlate1`) "OpacityTexture" "/Game/TimersClocksAndCountersPack/Textures/O_DialsAndCounters01Off.O_DialsAndCounters01Off")
  (`MaterialInstanceDynamic.SetTextureParameterValue` (`self.DynMatPlate2`) "OpacityTexture" "/Game/TimersClocksAndCountersPack/Textures/O_DialsAndCounters01Off.O_DialsAndCounters01Off")
  (`MaterialInstanceDynamic.SetTextureParameterValue` (`self.DynMatPlate3`) "OpacityTexture" "/Game/TimersClocksAndCountersPack/Textures/O_DialsAndCounters01Off.O_DialsAndCounters01Off")
  (`MaterialInstanceDynamic.SetTextureParameterValue` (`self.DynMatPlate4`) "OpacityTexture" "/Game/TimersClocksAndCountersPack/Textures/O_DialsAndCounters01Off.O_DialsAndCounters01Off")
  (`MaterialInstanceDynamic.SetTextureParameterValue` (`self.DynMatPlate5`) "OpacityTexture" "/Game/TimersClocksAndCountersPack/Textures/O_DialsAndCounters01Off.O_DialsAndCounters01Off")
  (`MaterialInstanceDynamic.SetTextureParameterValue` (`self.DynMatPlate6`) "OpacityTexture" "/Game/TimersClocksAndCountersPack/Textures/O_DialsAndCounters01Off.O_DialsAndCounters01Off")
  (`MaterialInstanceDynamic.SetTextureParameterValue` (`self.DynMatPlate7`) "OpacityTexture" "/Game/TimersClocksAndCountersPack/Textures/O_DialsAndCounters01Off.O_DialsAndCounters01Off")
  (`MaterialInstanceDynamic.SetTextureParameterValue` (`self.DynMatPlate8`) "OpacityTexture" "/Game/TimersClocksAndCountersPack/Textures/O_DialsAndCounters01Off.O_DialsAndCounters01Off")
  (`MaterialInstanceDynamic.SetTextureParameterValue` (`self.DynMatPlate9`) "OpacityTexture" "/Game/TimersClocksAndCountersPack/Textures/O_DialsAndCounters01Off.O_DialsAndCounters01Off")
  (`MaterialInstanceDynamic.SetTextureParameterValue` (`self.DynMatPlateColon`) "OpacityTexture" "/Game/TimersClocksAndCountersPack/Textures/O_DialsAndCounters01Off.O_DialsAndCounters01Off")
  (`MaterialInstanceDynamic.SetVectorParameterValue` _dynmatplate0 "EmissiveColor" (`self.GlowColor`))
  (`MaterialInstanceDynamic.SetVectorParameterValue` (`self.DynMatPlate1`) "EmissiveColor" (`self.GlowColor`))
  (`MaterialInstanceDynamic.SetVectorParameterValue` (`self.DynMatPlate2`) "EmissiveColor" (`self.GlowColor`))
  (`MaterialInstanceDynamic.SetVectorParameterValue` (`self.DynMatPlate3`) "EmissiveColor" (`self.GlowColor`))
  (`MaterialInstanceDynamic.SetVectorParameterValue` (`self.DynMatPlate4`) "EmissiveColor" (`self.GlowColor`))
  (`MaterialInstanceDynamic.SetVectorParameterValue` (`self.DynMatPlate5`) "EmissiveColor" (`self.GlowColor`))
  (`MaterialInstanceDynamic.SetVectorParameterValue` (`self.DynMatPlate6`) "EmissiveColor" (`self.GlowColor`))
  (`MaterialInstanceDynamic.SetVectorParameterValue` (`self.DynMatPlate7`) "EmissiveColor" (`self.GlowColor`))
  (`MaterialInstanceDynamic.SetVectorParameterValue` (`self.DynMatPlate8`) "EmissiveColor" (`self.GlowColor`))
  (`MaterialInstanceDynamic.SetVectorParameterValue` (`self.DynMatPlate9`) "EmissiveColor" (`self.GlowColor`))
  (`MaterialInstanceDynamic.SetVectorParameterValue` (`self.DynMatPlateColon`) "EmissiveColor" (`self.GlowColor`))
  (`MaterialInstanceDynamic.SetScalarParameterValue` _dynmatplate0 "EmissiveBrightness" 0.0)
  (`MaterialInstanceDynamic.SetScalarParameterValue` (`self.DynMatPlate1`) "EmissiveBrightness" 0.0)
  (`MaterialInstanceDynamic.SetScalarParameterValue` (`self.DynMatPlate2`) "EmissiveBrightness" 0.0)
  (`MaterialInstanceDynamic.SetScalarParameterValue` (`self.DynMatPlate3`) "EmissiveBrightness" 0.0)
  (`MaterialInstanceDynamic.SetScalarParameterValue` (`self.DynMatPlate9`) "EmissiveBrightness" 0.0)
  (`MaterialInstanceDynamic.SetScalarParameterValue` (`self.DynMatPlate8`) "EmissiveBrightness" 0.0)
  (`MaterialInstanceDynamic.SetScalarParameterValue` (`self.DynMatPlate6`) "EmissiveBrightness" 0.0)
  (`MaterialInstanceDynamic.SetScalarParameterValue` (`self.DynMatPlate7`) "EmissiveBrightness" 0.0)
  (`MaterialInstanceDynamic.SetScalarParameterValue` (`self.DynMatPlate5`) "EmissiveBrightness" 0.0)
  (`MaterialInstanceDynamic.SetScalarParameterValue` (`self.DynMatPlate4`) "EmissiveBrightness" 0.0)
  (`MaterialInstanceDynamic.SetScalarParameterValue` (`self.DynMatPlateColon`) "EmissiveBrightness" 0.0)
  (if (`self.IsColon`)
    (`MaterialInstanceDynamic.SetScalarParameterValue` _dynmatplatecolon "EmissiveBrightness" 200.0)
    (`MaterialInstanceDynamic.SetTextureParameterValue` _dynmatplatecolon "OpacityTexture" "/Game/TimersClocksAndCountersPack/Textures/O_DialsAndCounters01On.O_DialsAndCounters01On")
    (else
      (`MaterialInstanceDynamic.SetScalarParameterValue` _returnvalue "EmissiveBrightness" (* (`self.GlowBrightness`) (select `int` _displaynumber :`0` 15.0 :`1` 1.0 :`2` 1.0 :`3` 1.0 :`4` 1.3 :`5` 2.0 :`6` 3.0 :`7` 5.0 :`8` 7.0 :`9` 8.0 :!type "Float (single-precision)")))
      (`MaterialInstanceDynamic.SetTextureParameterValue` _returnvalue "OpacityTexture" "/Game/TimersClocksAndCountersPack/Textures/O_DialsAndCounters01On.O_DialsAndCounters01On"))))