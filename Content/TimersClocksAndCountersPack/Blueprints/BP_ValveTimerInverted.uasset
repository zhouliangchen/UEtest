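; Countdown timer prop that shows HH:MM or MM:SS on four BP_ValveDisplay child actors plus a colon valve.
; A gated Delay loop decrements once per minute or second by TimerType, pushes digits to the valves and fires EventTimerRunOut at zero.
; Events start, stop, reset and refresh the timer.
; The construction script previews the initial time and applies mesh variants, dynamic materials and valve glow settings.
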(event `self.ReceiveBeginPlay`
  (bind _customtimecacheb (`self.CustomTimeCacheB`))
  (bind _customtimecachea (`self.CustomTimeCacheA`))
  (bind _customtimecacheb_2 (`self.CustomTimeCacheB`))
  (bind _customtimecachea_2 (`self.CustomTimeCacheA`))
  (bind _returnvalue (/ _customtimecachea 10))
  (bind _returnvalue_2 (/ _customtimecacheb_2 10))
  (set `self.CustomTimeCacheA` (select `/Game/TimersClocksAndCountersPack/Enum_TimerType` (`self.TimerType`) :`NewEnumerator0` (`self.InitialTimeHours`) :`NewEnumerator1` (`self.InitialTimeMinutes`)))
  (set `self.CustomTimeCacheB` (select `/Game/TimersClocksAndCountersPack/Enum_TimerType` (`self.TimerType`) :`NewEnumerator0` (`self.InitialTimeMinutes`) :`NewEnumerator1` (`self.InitialTimeSeconds`)))
  ;[1 1 1] Run the Timer
  (`/Engine/EditorBlueprintResources/StandardMacros.Gate` (not (`self.AutoStartTimer`)) :!label _label
    (:`Exit`
      (`KismetSystemLibrary.Delay` (select `/Game/TimersClocksAndCountersPack/Enum_TimerType` (`self.TimerType`) :`NewEnumerator0` 60.0 :`NewEnumerator1` 1.0 :!type "Float (single-precision)"))
      (if (> _customtimecacheb 0)
        (`/Engine/EditorBlueprintResources/StandardMacros.DecrementInt` _customtimecacheb
          (:`  `
            (if (not (or (!= _customtimecacheb 0) (!= _customtimecachea_2 0))) :!label _label_2
              (`self.EventTimerRunOut`))
            (bind _asbp_valve_display (cast `/Game/TimersClocksAndCountersPack/Blueprints/BP_ValveDisplay` (`ChildActorComponent.ChildActor` (`self.HourA`))))
            (set `/Game/TimersClocksAndCountersPack/Blueprints/BP_ValveDisplay.DisplayNumber` _returnvalue _asbp_valve_display)
            (`/Game/TimersClocksAndCountersPack/Blueprints/BP_ValveDisplay.EventApplyValue` _asbp_valve_display)
            (bind _asbp_valve_display_2 (cast `/Game/TimersClocksAndCountersPack/Blueprints/BP_ValveDisplay` (`ChildActorComponent.ChildActor` (`self.HourB`))))
            (set `/Game/TimersClocksAndCountersPack/Blueprints/BP_ValveDisplay.DisplayNumber` (- _customtimecachea (* _returnvalue 10)) _asbp_valve_display_2)
            (`/Game/TimersClocksAndCountersPack/Blueprints/BP_ValveDisplay.EventApplyValue` _asbp_valve_display_2)
            (bind _asbp_valve_display_3 (cast `/Game/TimersClocksAndCountersPack/Blueprints/BP_ValveDisplay` (`ChildActorComponent.ChildActor` (`self.MinA`))))
            (set `/Game/TimersClocksAndCountersPack/Blueprints/BP_ValveDisplay.DisplayNumber` _returnvalue_2 _asbp_valve_display_3)
            (`/Game/TimersClocksAndCountersPack/Blueprints/BP_ValveDisplay.EventApplyValue` _asbp_valve_display_3)
            (bind _asbp_valve_display_4 (cast `/Game/TimersClocksAndCountersPack/Blueprints/BP_ValveDisplay` (`ChildActorComponent.ChildActor` (`self.MinB`))))
            (set `/Game/TimersClocksAndCountersPack/Blueprints/BP_ValveDisplay.DisplayNumber` (- _customtimecacheb_2 (* _returnvalue_2 10)) _asbp_valve_display_4)
            (`/Game/TimersClocksAndCountersPack/Blueprints/BP_ValveDisplay.EventApplyValue` _asbp_valve_display_4)
            (goto _label)))
        (elif (> _customtimecachea_2 0)
          (`/Engine/EditorBlueprintResources/StandardMacros.DecrementInt` _customtimecachea_2
            (:`  `
              (set `self.CustomTimeCacheB` 59)
              (goto _label_2))))))))

(event `StartTimer`
  ;[1 1 1] Call the Start Timer or Stop Timer Events to start/stop the timer during gameplay
  (`|ExecutionSequence`
    (:`then_0`
      (goto _label :!via `Open`))
    (:`then_1`
      (goto _label))))

(event `StopTimer`
  ;[1 1 1] Call the Start Timer or Stop Timer Events to start/stop the timer during gameplay
  (goto _label :!via `Close`))

(event `EventResetTimer`
  ;[1 1 1] Reset timer to initial value
  (set `self.CustomTimeCacheA` (select `/Game/TimersClocksAndCountersPack/Enum_TimerType` (`self.TimerType`) :`NewEnumerator0` (`self.InitialTimeHours`) :`NewEnumerator1` (`self.InitialTimeMinutes`)))
  (set `self.CustomTimeCacheB` (select `/Game/TimersClocksAndCountersPack/Enum_TimerType` (`self.TimerType`) :`NewEnumerator0` (`self.InitialTimeMinutes`) :`NewEnumerator1` (`self.InitialTimeSeconds`)))
  (set `self.IsTimerZero` false)
  (`self.EventUpdateDisplay`))

(event `EventTimerRunOut`
  ;[1 1 1] This custom event is triggered when the timer reaches zero
  (set `self.IsTimerZero` true))

(event `EventUpdateDisplay`
  (bind _customtimecachea (`self.CustomTimeCacheA`))
  (bind _customtimecacheb (`self.CustomTimeCacheB`))
  (bind _returnvalue (/ _customtimecacheb 10))
  (bind _returnvalue_2 (/ _customtimecachea 10))
  ;[1 1 1] Call this event to manually update the display
  (bind _asbp_valve_display (cast `/Game/TimersClocksAndCountersPack/Blueprints/BP_ValveDisplay` (`ChildActorComponent.ChildActor` (`self.HourA`))))
  (set `/Game/TimersClocksAndCountersPack/Blueprints/BP_ValveDisplay.DisplayNumber` _returnvalue_2 _asbp_valve_display)
  (`/Game/TimersClocksAndCountersPack/Blueprints/BP_ValveDisplay.EventApplyValue` _asbp_valve_display)
  (bind _asbp_valve_display_2 (cast `/Game/TimersClocksAndCountersPack/Blueprints/BP_ValveDisplay` (`ChildActorComponent.ChildActor` (`self.HourB`))))
  (set `/Game/TimersClocksAndCountersPack/Blueprints/BP_ValveDisplay.DisplayNumber` (- _customtimecachea (* _returnvalue_2 10)) _asbp_valve_display_2)
  (`/Game/TimersClocksAndCountersPack/Blueprints/BP_ValveDisplay.EventApplyValue` _asbp_valve_display_2)
  (bind _asbp_valve_display_3 (cast `/Game/TimersClocksAndCountersPack/Blueprints/BP_ValveDisplay` (`ChildActorComponent.ChildActor` (`self.MinA`))))
  (set `/Game/TimersClocksAndCountersPack/Blueprints/BP_ValveDisplay.DisplayNumber` _returnvalue _asbp_valve_display_3)
  (`/Game/TimersClocksAndCountersPack/Blueprints/BP_ValveDisplay.EventApplyValue` _asbp_valve_display_3)
  (bind _asbp_valve_display_4 (cast `/Game/TimersClocksAndCountersPack/Blueprints/BP_ValveDisplay` (`ChildActorComponent.ChildActor` (`self.MinB`))))
  (set `/Game/TimersClocksAndCountersPack/Blueprints/BP_ValveDisplay.DisplayNumber` (- _customtimecacheb (* _returnvalue 10)) _asbp_valve_display_4)
  (`/Game/TimersClocksAndCountersPack/Blueprints/BP_ValveDisplay.EventApplyValue` _asbp_valve_display_4))

(fn `UserConstructionScript`
  (bind _addsocket (`self.AddSocket`))
  (bind _sm_socket04 (`self.SM_Socket04`))
  (bind _displayglowbrightness (`self.DisplayGlowBrightness`))
  (bind _shieldvariation (`self.ShieldVariation`))
  (bind _sm_shield01 (`self.SM_Shield01`))
  (bind _basevariation (`self.BaseVariation`))
  (bind _sm_valvebase01 (`self.SM_ValveBase01`))
  (bind _displayglowbrightness_2 (`self.DisplayGlowBrightness`))
  (bind _displayglowbrightness_3 (`self.DisplayGlowBrightness`))
  (bind _displayglowbrightness_4 (`self.DisplayGlowBrightness`))
  (bind _displayglowbrightness_5 (`self.DisplayGlowBrightness`))
  (bind _returnvalue (!= _shieldvariation 0))
  (bind _returnvalue_2 (!= _basevariation 0))
  (bind _returnvalue_3 (select `/Game/TimersClocksAndCountersPack/Enum_TimerType` (`self.TimerType`) :`NewEnumerator0` (`self.InitialTimeMinutes`) :`NewEnumerator1` (`self.InitialTimeSeconds`)))
  (bind _returnvalue_4 (select `/Game/TimersClocksAndCountersPack/Enum_TimerType` (`self.TimerType`) :`NewEnumerator0` (`self.InitialTimeHours`) :`NewEnumerator1` (`self.InitialTimeMinutes`)))
  (bind _returnvalue_5 (/ _returnvalue_3 10))
  (bind _returnvalue_6 (/ _returnvalue_4 10))
  ;[1 1 1] Get System time and apply correct values to all displays
  (bind _asbp_valve_display (cast `/Game/TimersClocksAndCountersPack/Blueprints/BP_ValveDisplay` (`ChildActorComponent.ChildActor` (`self.HourA`))))
  (set `/Game/TimersClocksAndCountersPack/Blueprints/BP_ValveDisplay.DisplayNumber` _returnvalue_6 _asbp_valve_display)
  (`/Game/TimersClocksAndCountersPack/Blueprints/BP_ValveDisplay.EventApplyValue` _asbp_valve_display)
  (bind _asbp_valve_display_2 (cast `/Game/TimersClocksAndCountersPack/Blueprints/BP_ValveDisplay` (`ChildActorComponent.ChildActor` (`self.HourB`))))
  (set `/Game/TimersClocksAndCountersPack/Blueprints/BP_ValveDisplay.DisplayNumber` (- _returnvalue_4 (* _returnvalue_6 10)) _asbp_valve_display_2)
  (`/Game/TimersClocksAndCountersPack/Blueprints/BP_ValveDisplay.EventApplyValue` _asbp_valve_display_2)
  (bind _asbp_valve_display_3 (cast `/Game/TimersClocksAndCountersPack/Blueprints/BP_ValveDisplay` (`ChildActorComponent.ChildActor` (`self.MinA`))))
  (set `/Game/TimersClocksAndCountersPack/Blueprints/BP_ValveDisplay.DisplayNumber` _returnvalue_5 _asbp_valve_display_3)
  (`/Game/TimersClocksAndCountersPack/Blueprints/BP_ValveDisplay.EventApplyValue` _asbp_valve_display_3)
  (bind _asbp_valve_display_4 (cast `/Game/TimersClocksAndCountersPack/Blueprints/BP_ValveDisplay` (`ChildActorComponent.ChildActor` (`self.MinB`))))
  (set `/Game/TimersClocksAndCountersPack/Blueprints/BP_ValveDisplay.DisplayNumber` (- _returnvalue_3 (* _returnvalue_5 10)) _asbp_valve_display_4)
  (`/Game/TimersClocksAndCountersPack/Blueprints/BP_ValveDisplay.EventApplyValue` _asbp_valve_display_4)
  ;[1 1 1] Apply settings as set by the user
  (`StaticMeshComponent.SetStaticMesh` _sm_valvebase01 (select `int` _basevariation :`0` "/Game/TimersClocksAndCountersPack/Meshes/SM_ValveBase01.SM_ValveBase01" :`1` "/Game/TimersClocksAndCountersPack/Meshes/SM_ValveBase01.SM_ValveBase01" :`2` "/Game/TimersClocksAndCountersPack/Meshes/SM_ValveBase02.SM_ValveBase02" :!type "StaticMesh Object Reference"))
  (`SceneComponent.SetVisibility` _sm_valvebase01 _returnvalue_2 false)
  (`PrimitiveComponent.SetCastShadow` _sm_valvebase01 _returnvalue_2)
  (`SceneComponent.SetVisibility` _sm_socket04 _addsocket false)
  (`SceneComponent.SetVisibility` (`self.SM_Socket02`) _addsocket false)
  (`SceneComponent.SetVisibility` (`self.SM_Socket05`) _addsocket false)
  (`SceneComponent.SetVisibility` (`self.SM_Socket03`) _addsocket false)
  (`SceneComponent.SetVisibility` (`self.SM_Socket01`) _addsocket false)
  (`PrimitiveComponent.SetCastShadow` _sm_socket04 _addsocket)
  (`PrimitiveComponent.SetCastShadow` (`self.SM_Socket02`) _addsocket)
  (`PrimitiveComponent.SetCastShadow` (`self.SM_Socket05`) _addsocket)
  (`PrimitiveComponent.SetCastShadow` (`self.SM_Socket03`) _addsocket)
  (`PrimitiveComponent.SetCastShadow` (`self.SM_Socket01`) _addsocket)
  (bind _returnvalue_7 (`KismetMaterialLibrary.CreateDynamicMaterialInstance` "/Game/TimersClocksAndCountersPack/Materials/M_Bases01_Inst.M_Bases01_Inst"))
  (bind _output_get (set `self.DynMatBase` _returnvalue_7))
  (`PrimitiveComponent.SetMaterial` (`self.SM_ValveBase01`) 0 _output_get)
  (`MaterialInstanceDynamic.SetScalarParameterValue` _output_get "New-Old" (`self.AgeBase`))
  (`MaterialInstanceDynamic.SetScalarParameterValue` _output_get "Metallic" (`self.MetallicBase`))
  (`MaterialInstanceDynamic.SetScalarParameterValue` _output_get "FadeOutTexture" (`self.FadeOutTextureBase`))
  (`MaterialInstanceDynamic.SetScalarParameterValue` _output_get "DesaturateTexture" (`self.DesaturateTextureBase`))
  (`MaterialInstanceDynamic.SetScalarParameterValue` _output_get "Specular" (`self.SpecularBase`))
  (`MaterialInstanceDynamic.SetScalarParameterValue` _output_get "Roughness" (`self.RoughnessBase`))
  (`MaterialInstanceDynamic.SetVectorParameterValue` _output_get "Tint" (`self.TintBase`))
  (`MaterialInstanceDynamic.SetScalarParameterValue` _output_get "NormalMapStrength" (`self.NormalMapStrengthBase`))
  (bind _returnvalue_8 (`KismetMaterialLibrary.CreateDynamicMaterialInstance` "/Game/TimersClocksAndCountersPack/Materials/M_CounterMetal01_Inst.M_CounterMetal01_Inst"))
  (bind _output_get_2 (set `self.DynMatSocketShield` _returnvalue_8))
  (`PrimitiveComponent.SetMaterial` (`self.SM_Socket01`) 0 _output_get_2)
  (`PrimitiveComponent.SetMaterial` (`self.SM_Socket04`) 0 _output_get_2)
  (`PrimitiveComponent.SetMaterial` (`self.SM_Socket02`) 0 _output_get_2)
  (`PrimitiveComponent.SetMaterial` (`self.SM_Socket03`) 0 _output_get_2)
  (`PrimitiveComponent.SetMaterial` (`self.SM_Socket05`) 0 _output_get_2)
  (`PrimitiveComponent.SetMaterial` (`self.SM_Shield01`) 0 _output_get_2)
  (`MaterialInstanceDynamic.SetVectorParameterValue` _output_get_2 "Tint" (`self.TintSocketsAndShield`))
  (`MaterialInstanceDynamic.SetScalarParameterValue` _output_get_2 "New-Old" (`self.AgeSocketsAndShield`))
  (`MaterialInstanceDynamic.SetScalarParameterValue` _output_get_2 "Metallic" (`self.MetallicSocketsAndShield`))
  (`MaterialInstanceDynamic.SetScalarParameterValue` _output_get_2 "Roughness" (`self.RoughnessSocketsAndShield`))
  (`MaterialInstanceDynamic.SetScalarParameterValue` _output_get_2 "Specular" (`self.SpecularSocketsAndShield`))
  (`MaterialInstanceDynamic.SetScalarParameterValue` _output_get_2 "NormalMapStrength" (`self.NormalMapStrengthSocketsAndShield`))
  (`StaticMeshComponent.SetStaticMesh` _sm_shield01 (select `int` _shieldvariation :`0` "/Game/TimersClocksAndCountersPack/Meshes/SM_Shield01.SM_Shield01" :`1` "/Game/TimersClocksAndCountersPack/Meshes/SM_Shield01.SM_Shield01" :`2` "/Game/TimersClocksAndCountersPack/Meshes/SM_Shield02.SM_Shield02" :`3` "/Game/TimersClocksAndCountersPack/Meshes/SM_Shield03.SM_Shield03" :!type "StaticMesh Object Reference"))
  (`SceneComponent.SetVisibility` _sm_shield01 _returnvalue false)
  (`PrimitiveComponent.SetCastShadow` _sm_shield01 _returnvalue)
  ;[1 1 1] Apply settings to each valve
  (`|ExecutionSequence`
    (:`then_0`
      (bind _asbp_valve_display_5 (cast `/Game/TimersClocksAndCountersPack/Blueprints/BP_ValveDisplay` (`ChildActorComponent.ChildActor` (`self.HourA`))))
      (bind _dynmatvalveglass (`/Game/TimersClocksAndCountersPack/Blueprints/BP_ValveDisplay.DynMatValveGlass` _asbp_valve_display_5))
      (`MaterialInstanceDynamic.SetScalarParameterValue` _dynmatvalveglass "New-Old" (`self.AgeValve`))
      (`MaterialInstanceDynamic.SetScalarParameterValue` (`/Game/TimersClocksAndCountersPack/Blueprints/BP_ValveDisplay.DynMatValveEnds` _asbp_valve_display_5) "New-Old" (`self.AgeValve`))
      (`MaterialInstanceDynamic.SetScalarParameterValue` _dynmatvalveglass "Roughness" (`self.RoughnessValve`))
      (`MaterialInstanceDynamic.SetScalarParameterValue` (`/Game/TimersClocksAndCountersPack/Blueprints/BP_ValveDisplay.DynMatValveEnds` _asbp_valve_display_5) "Roughness" (`self.RoughnessValve`))
      (`MaterialInstanceDynamic.SetScalarParameterValue` _dynmatvalveglass "Specular" (`self.SpecularValve`))
      (`MaterialInstanceDynamic.SetScalarParameterValue` (`/Game/TimersClocksAndCountersPack/Blueprints/BP_ValveDisplay.DynMatValveEnds` _asbp_valve_display_5) "Specular" (`self.SpecularValve`))
      (`MaterialInstanceDynamic.SetScalarParameterValue` _dynmatvalveglass "Metallic" (`self.MetallicValve`))
      (`MaterialInstanceDynamic.SetScalarParameterValue` (`/Game/TimersClocksAndCountersPack/Blueprints/BP_ValveDisplay.DynMatValveEnds` _asbp_valve_display_5) "Metallic" (`self.MetallicValve`))
      (`MaterialInstanceDynamic.SetScalarParameterValue` _dynmatvalveglass "Normalmapstrength" (`self.NormalMapStrengthValve`))
      (`MaterialInstanceDynamic.SetScalarParameterValue` (`/Game/TimersClocksAndCountersPack/Blueprints/BP_ValveDisplay.DynMatValveEnds` _asbp_valve_display_5) "Normalmapstrength" (`self.NormalMapStrengthValve`))
      (`MaterialInstanceDynamic.SetScalarParameterValue` _dynmatvalveglass "ReflactiveIndex" (`self.RefractionValveGlass`))
      (`MaterialInstanceDynamic.SetScalarParameterValue` (`/Game/TimersClocksAndCountersPack/Blueprints/BP_ValveDisplay.DynMatValveEnds` _asbp_valve_display_5) "ReflactiveIndex" (`self.RefractionValveGlass`))
      (`MaterialInstanceDynamic.SetScalarParameterValue` _dynmatvalveglass "DesaturateTexture" (`self.ValveDesaturateTexture`))
      (`MaterialInstanceDynamic.SetScalarParameterValue` (`/Game/TimersClocksAndCountersPack/Blueprints/BP_ValveDisplay.DynMatValveEnds` _asbp_valve_display_5) "DesaturateTexture" (`self.ValveDesaturateTexture`))
      (bind _dynmatplate9 (`/Game/TimersClocksAndCountersPack/Blueprints/BP_ValveDisplay.DynMatPlate9` _asbp_valve_display_5))
      (`MaterialInstanceDynamic.SetVectorParameterValue` _dynmatplate9 "EmissiveColor" (`self.DisplayGlowColor`))
      (`MaterialInstanceDynamic.SetVectorParameterValue` (`/Game/TimersClocksAndCountersPack/Blueprints/BP_ValveDisplay.DynMatPlate0` _asbp_valve_display_5) "EmissiveColor" (`self.DisplayGlowColor`))
      (`MaterialInstanceDynamic.SetVectorParameterValue` (`/Game/TimersClocksAndCountersPack/Blueprints/BP_ValveDisplay.DynMatPlate1` _asbp_valve_display_5) "EmissiveColor" (`self.DisplayGlowColor`))
      (`MaterialInstanceDynamic.SetVectorParameterValue` (`/Game/TimersClocksAndCountersPack/Blueprints/BP_ValveDisplay.DynMatPlate2` _asbp_valve_display_5) "EmissiveColor" (`self.DisplayGlowColor`))
      (`MaterialInstanceDynamic.SetVectorParameterValue` (`/Game/TimersClocksAndCountersPack/Blueprints/BP_ValveDisplay.DynMatPlate3` _asbp_valve_display_5) "EmissiveColor" (`self.DisplayGlowColor`))
      (`MaterialInstanceDynamic.SetVectorParameterValue` (`/Game/TimersClocksAndCountersPack/Blueprints/BP_ValveDisplay.DynMatPlate4` _asbp_valve_display_5) "EmissiveColor" (`self.DisplayGlowColor`))
      (`MaterialInstanceDynamic.SetVectorParameterValue` (`/Game/TimersClocksAndCountersPack/Blueprints/BP_ValveDisplay.DynMatPlate5` _asbp_valve_display_5) "EmissiveColor" (`self.DisplayGlowColor`))
      (`MaterialInstanceDynamic.SetVectorParameterValue` (`/Game/TimersClocksAndCountersPack/Blueprints/BP_ValveDisplay.DynMatPlate6` _asbp_valve_display_5) "EmissiveColor" (`self.DisplayGlowColor`))
      (`MaterialInstanceDynamic.SetVectorParameterValue` (`/Game/TimersClocksAndCountersPack/Blueprints/BP_ValveDisplay.DynMatPlate7` _asbp_valve_display_5) "EmissiveColor" (`self.DisplayGlowColor`))
      (`MaterialInstanceDynamic.SetVectorParameterValue` (`/Game/TimersClocksAndCountersPack/Blueprints/BP_ValveDisplay.DynMatPlate8` _asbp_valve_display_5) "EmissiveColor" (`self.DisplayGlowColor`))
      (`MaterialInstanceDynamic.SetVectorParameterValue` (`/Game/TimersClocksAndCountersPack/Blueprints/BP_ValveDisplay.DynMatPlateColon` _asbp_valve_display_5) "EmissiveColor" (`self.DisplayGlowColor`))
      (if (`/Game/TimersClocksAndCountersPack/Blueprints/BP_ValveDisplay.IsColon` _asbp_valve_display_5)
        (`MaterialInstanceDynamic.SetScalarParameterValue` (`/Game/TimersClocksAndCountersPack/Blueprints/BP_ValveDisplay.DynMatPlateColon` _asbp_valve_display_5) "EmissiveBrightness" (* _displayglowbrightness_3 2.0))
        (else
          (set `/Game/TimersClocksAndCountersPack/Blueprints/BP_ValveDisplay.GlowBrightness` _displayglowbrightness_3 _asbp_valve_display_5)
          (bind _displaynumber (`/Game/TimersClocksAndCountersPack/Blueprints/BP_ValveDisplay.DisplayNumber` _asbp_valve_display_5))
          (`MaterialInstanceDynamic.SetScalarParameterValue` (select `int` _displaynumber :`0` (`/Game/TimersClocksAndCountersPack/Blueprints/BP_ValveDisplay.DynMatPlate0` _asbp_valve_display_5) :`1` (`/Game/TimersClocksAndCountersPack/Blueprints/BP_ValveDisplay.DynMatPlate1` _asbp_valve_display_5) :`2` (`/Game/TimersClocksAndCountersPack/Blueprints/BP_ValveDisplay.DynMatPlate2` _asbp_valve_display_5) :`3` (`/Game/TimersClocksAndCountersPack/Blueprints/BP_ValveDisplay.DynMatPlate3` _asbp_valve_display_5) :`4` (`/Game/TimersClocksAndCountersPack/Blueprints/BP_ValveDisplay.DynMatPlate4` _asbp_valve_display_5) :`5` (`/Game/TimersClocksAndCountersPack/Blueprints/BP_ValveDisplay.DynMatPlate5` _asbp_valve_display_5) :`6` (`/Game/TimersClocksAndCountersPack/Blueprints/BP_ValveDisplay.DynMatPlate6` _asbp_valve_display_5) :`7` (`/Game/TimersClocksAndCountersPack/Blueprints/BP_ValveDisplay.DynMatPlate7` _asbp_valve_display_5) :`8` (`/Game/TimersClocksAndCountersPack/Blueprints/BP_ValveDisplay.DynMatPlate8` _asbp_valve_display_5) :`9` _dynmatplate9) "EmissiveBrightness" (* (`self.DisplayGlowBrightness`) (select `int` _displaynumber :`0` 11.0 :`1` 1.0 :`2` 1.0 :`3` 1.0 :`4` 1.3 :`5` 2.0 :`6` 3.0 :`7` 5.0 :`8` 7.0 :`9` 8.0 :!type "Float (single-precision)"))))))
    (:`then_1`
      (bind _asbp_valve_display_6 (cast `/Game/TimersClocksAndCountersPack/Blueprints/BP_ValveDisplay` (`ChildActorComponent.ChildActor` (`self.HourB`))))
      (bind _dynmatvalveglass_2 (`/Game/TimersClocksAndCountersPack/Blueprints/BP_ValveDisplay.DynMatValveGlass` _asbp_valve_display_6))
      (`MaterialInstanceDynamic.SetScalarParameterValue` _dynmatvalveglass_2 "New-Old" (`self.AgeValve`))
      (`MaterialInstanceDynamic.SetScalarParameterValue` (`/Game/TimersClocksAndCountersPack/Blueprints/BP_ValveDisplay.DynMatValveEnds` _asbp_valve_display_6) "New-Old" (`self.AgeValve`))
      (`MaterialInstanceDynamic.SetScalarParameterValue` _dynmatvalveglass_2 "Roughness" (`self.RoughnessValve`))
      (`MaterialInstanceDynamic.SetScalarParameterValue` (`/Game/TimersClocksAndCountersPack/Blueprints/BP_ValveDisplay.DynMatValveEnds` _asbp_valve_display_6) "Roughness" (`self.RoughnessValve`))
      (`MaterialInstanceDynamic.SetScalarParameterValue` _dynmatvalveglass_2 "Specular" (`self.SpecularValve`))
      (`MaterialInstanceDynamic.SetScalarParameterValue` (`/Game/TimersClocksAndCountersPack/Blueprints/BP_ValveDisplay.DynMatValveEnds` _asbp_valve_display_6) "Specular" (`self.SpecularValve`))
      (`MaterialInstanceDynamic.SetScalarParameterValue` _dynmatvalveglass_2 "Metallic" (`self.MetallicValve`))
      (`MaterialInstanceDynamic.SetScalarParameterValue` (`/Game/TimersClocksAndCountersPack/Blueprints/BP_ValveDisplay.DynMatValveEnds` _asbp_valve_display_6) "Metallic" (`self.MetallicValve`))
      (`MaterialInstanceDynamic.SetScalarParameterValue` _dynmatvalveglass_2 "Normalmapstrength" (`self.NormalMapStrengthValve`))
      (`MaterialInstanceDynamic.SetScalarParameterValue` (`/Game/TimersClocksAndCountersPack/Blueprints/BP_ValveDisplay.DynMatValveEnds` _asbp_valve_display_6) "Normalmapstrength" (`self.NormalMapStrengthValve`))
      (`MaterialInstanceDynamic.SetScalarParameterValue` _dynmatvalveglass_2 "ReflactiveIndex" (`self.RefractionValveGlass`))
      (`MaterialInstanceDynamic.SetScalarParameterValue` (`/Game/TimersClocksAndCountersPack/Blueprints/BP_ValveDisplay.DynMatValveEnds` _asbp_valve_display_6) "ReflactiveIndex" (`self.RefractionValveGlass`))
      (`MaterialInstanceDynamic.SetScalarParameterValue` _dynmatvalveglass_2 "DesaturateTexture" (`self.ValveDesaturateTexture`))
      (`MaterialInstanceDynamic.SetScalarParameterValue` (`/Game/TimersClocksAndCountersPack/Blueprints/BP_ValveDisplay.DynMatValveEnds` _asbp_valve_display_6) "DesaturateTexture" (`self.ValveDesaturateTexture`))
      (bind _dynmatplate9_2 (`/Game/TimersClocksAndCountersPack/Blueprints/BP_ValveDisplay.DynMatPlate9` _asbp_valve_display_6))
      (`MaterialInstanceDynamic.SetVectorParameterValue` _dynmatplate9_2 "EmissiveColor" (`self.DisplayGlowColor`))
      (`MaterialInstanceDynamic.SetVectorParameterValue` (`/Game/TimersClocksAndCountersPack/Blueprints/BP_ValveDisplay.DynMatPlate0` _asbp_valve_display_6) "EmissiveColor" (`self.DisplayGlowColor`))
      (`MaterialInstanceDynamic.SetVectorParameterValue` (`/Game/TimersClocksAndCountersPack/Blueprints/BP_ValveDisplay.DynMatPlate1` _asbp_valve_display_6) "EmissiveColor" (`self.DisplayGlowColor`))
      (`MaterialInstanceDynamic.SetVectorParameterValue` (`/Game/TimersClocksAndCountersPack/Blueprints/BP_ValveDisplay.DynMatPlate2` _asbp_valve_display_6) "EmissiveColor" (`self.DisplayGlowColor`))
      (`MaterialInstanceDynamic.SetVectorParameterValue` (`/Game/TimersClocksAndCountersPack/Blueprints/BP_ValveDisplay.DynMatPlate3` _asbp_valve_display_6) "EmissiveColor" (`self.DisplayGlowColor`))
      (`MaterialInstanceDynamic.SetVectorParameterValue` (`/Game/TimersClocksAndCountersPack/Blueprints/BP_ValveDisplay.DynMatPlate4` _asbp_valve_display_6) "EmissiveColor" (`self.DisplayGlowColor`))
      (`MaterialInstanceDynamic.SetVectorParameterValue` (`/Game/TimersClocksAndCountersPack/Blueprints/BP_ValveDisplay.DynMatPlate5` _asbp_valve_display_6) "EmissiveColor" (`self.DisplayGlowColor`))
      (`MaterialInstanceDynamic.SetVectorParameterValue` (`/Game/TimersClocksAndCountersPack/Blueprints/BP_ValveDisplay.DynMatPlate6` _asbp_valve_display_6) "EmissiveColor" (`self.DisplayGlowColor`))
      (`MaterialInstanceDynamic.SetVectorParameterValue` (`/Game/TimersClocksAndCountersPack/Blueprints/BP_ValveDisplay.DynMatPlate7` _asbp_valve_display_6) "EmissiveColor" (`self.DisplayGlowColor`))
      (`MaterialInstanceDynamic.SetVectorParameterValue` (`/Game/TimersClocksAndCountersPack/Blueprints/BP_ValveDisplay.DynMatPlate8` _asbp_valve_display_6) "EmissiveColor" (`self.DisplayGlowColor`))
      (`MaterialInstanceDynamic.SetVectorParameterValue` (`/Game/TimersClocksAndCountersPack/Blueprints/BP_ValveDisplay.DynMatPlateColon` _asbp_valve_display_6) "EmissiveColor" (`self.DisplayGlowColor`))
      (if (`/Game/TimersClocksAndCountersPack/Blueprints/BP_ValveDisplay.IsColon` _asbp_valve_display_6)
        (`MaterialInstanceDynamic.SetScalarParameterValue` (`/Game/TimersClocksAndCountersPack/Blueprints/BP_ValveDisplay.DynMatPlateColon` _asbp_valve_display_6) "EmissiveBrightness" (* _displayglowbrightness_2 2.0))
        (else
          (set `/Game/TimersClocksAndCountersPack/Blueprints/BP_ValveDisplay.GlowBrightness` _displayglowbrightness_2 _asbp_valve_display_6)
          (bind _displaynumber_2 (`/Game/TimersClocksAndCountersPack/Blueprints/BP_ValveDisplay.DisplayNumber` _asbp_valve_display_6))
          (`MaterialInstanceDynamic.SetScalarParameterValue` (select `int` _displaynumber_2 :`0` (`/Game/TimersClocksAndCountersPack/Blueprints/BP_ValveDisplay.DynMatPlate0` _asbp_valve_display_6) :`1` (`/Game/TimersClocksAndCountersPack/Blueprints/BP_ValveDisplay.DynMatPlate1` _asbp_valve_display_6) :`2` (`/Game/TimersClocksAndCountersPack/Blueprints/BP_ValveDisplay.DynMatPlate2` _asbp_valve_display_6) :`3` (`/Game/TimersClocksAndCountersPack/Blueprints/BP_ValveDisplay.DynMatPlate3` _asbp_valve_display_6) :`4` (`/Game/TimersClocksAndCountersPack/Blueprints/BP_ValveDisplay.DynMatPlate4` _asbp_valve_display_6) :`5` (`/Game/TimersClocksAndCountersPack/Blueprints/BP_ValveDisplay.DynMatPlate5` _asbp_valve_display_6) :`6` (`/Game/TimersClocksAndCountersPack/Blueprints/BP_ValveDisplay.DynMatPlate6` _asbp_valve_display_6) :`7` (`/Game/TimersClocksAndCountersPack/Blueprints/BP_ValveDisplay.DynMatPlate7` _asbp_valve_display_6) :`8` (`/Game/TimersClocksAndCountersPack/Blueprints/BP_ValveDisplay.DynMatPlate8` _asbp_valve_display_6) :`9` _dynmatplate9_2) "EmissiveBrightness" (* (`self.DisplayGlowBrightness`) (select `int` _displaynumber_2 :`0` 11.0 :`1` 1.0 :`2` 1.0 :`3` 1.0 :`4` 1.3 :`5` 2.0 :`6` 3.0 :`7` 5.0 :`8` 7.0 :`9` 8.0 :!type "Float (single-precision)"))))))
    (:`then_2`
      (bind _asbp_valve_display_7 (cast `/Game/TimersClocksAndCountersPack/Blueprints/BP_ValveDisplay` (`ChildActorComponent.ChildActor` (`self.MinA`))))
      (bind _dynmatvalveglass_3 (`/Game/TimersClocksAndCountersPack/Blueprints/BP_ValveDisplay.DynMatValveGlass` _asbp_valve_display_7))
      (`MaterialInstanceDynamic.SetScalarParameterValue` _dynmatvalveglass_3 "New-Old" (`self.AgeValve`))
      (`MaterialInstanceDynamic.SetScalarParameterValue` (`/Game/TimersClocksAndCountersPack/Blueprints/BP_ValveDisplay.DynMatValveEnds` _asbp_valve_display_7) "New-Old" (`self.AgeValve`))
      (`MaterialInstanceDynamic.SetScalarParameterValue` _dynmatvalveglass_3 "Roughness" (`self.RoughnessValve`))
      (`MaterialInstanceDynamic.SetScalarParameterValue` (`/Game/TimersClocksAndCountersPack/Blueprints/BP_ValveDisplay.DynMatValveEnds` _asbp_valve_display_7) "Roughness" (`self.RoughnessValve`))
      (`MaterialInstanceDynamic.SetScalarParameterValue` _dynmatvalveglass_3 "Specular" (`self.SpecularValve`))
      (`MaterialInstanceDynamic.SetScalarParameterValue` (`/Game/TimersClocksAndCountersPack/Blueprints/BP_ValveDisplay.DynMatValveEnds` _asbp_valve_display_7) "Specular" (`self.SpecularValve`))
      (`MaterialInstanceDynamic.SetScalarParameterValue` _dynmatvalveglass_3 "Metallic" (`self.MetallicValve`))
      (`MaterialInstanceDynamic.SetScalarParameterValue` (`/Game/TimersClocksAndCountersPack/Blueprints/BP_ValveDisplay.DynMatValveEnds` _asbp_valve_display_7) "Metallic" (`self.MetallicValve`))
      (`MaterialInstanceDynamic.SetScalarParameterValue` _dynmatvalveglass_3 "Normalmapstrength" (`self.NormalMapStrengthValve`))
      (`MaterialInstanceDynamic.SetScalarParameterValue` (`/Game/TimersClocksAndCountersPack/Blueprints/BP_ValveDisplay.DynMatValveEnds` _asbp_valve_display_7) "Normalmapstrength" (`self.NormalMapStrengthValve`))
      (`MaterialInstanceDynamic.SetScalarParameterValue` _dynmatvalveglass_3 "ReflactiveIndex" (`self.RefractionValveGlass`))
      (`MaterialInstanceDynamic.SetScalarParameterValue` (`/Game/TimersClocksAndCountersPack/Blueprints/BP_ValveDisplay.DynMatValveEnds` _asbp_valve_display_7) "ReflactiveIndex" (`self.RefractionValveGlass`))
      (`MaterialInstanceDynamic.SetScalarParameterValue` _dynmatvalveglass_3 "DesaturateTexture" (`self.ValveDesaturateTexture`))
      (`MaterialInstanceDynamic.SetScalarParameterValue` (`/Game/TimersClocksAndCountersPack/Blueprints/BP_ValveDisplay.DynMatValveEnds` _asbp_valve_display_7) "DesaturateTexture" (`self.ValveDesaturateTexture`))
      (bind _dynmatplate9_3 (`/Game/TimersClocksAndCountersPack/Blueprints/BP_ValveDisplay.DynMatPlate9` _asbp_valve_display_7))
      (`MaterialInstanceDynamic.SetVectorParameterValue` _dynmatplate9_3 "EmissiveColor" (`self.DisplayGlowColor`))
      (`MaterialInstanceDynamic.SetVectorParameterValue` (`/Game/TimersClocksAndCountersPack/Blueprints/BP_ValveDisplay.DynMatPlate0` _asbp_valve_display_7) "EmissiveColor" (`self.DisplayGlowColor`))
      (`MaterialInstanceDynamic.SetVectorParameterValue` (`/Game/TimersClocksAndCountersPack/Blueprints/BP_ValveDisplay.DynMatPlate1` _asbp_valve_display_7) "EmissiveColor" (`self.DisplayGlowColor`))
      (`MaterialInstanceDynamic.SetVectorParameterValue` (`/Game/TimersClocksAndCountersPack/Blueprints/BP_ValveDisplay.DynMatPlate2` _asbp_valve_display_7) "EmissiveColor" (`self.DisplayGlowColor`))
      (`MaterialInstanceDynamic.SetVectorParameterValue` (`/Game/TimersClocksAndCountersPack/Blueprints/BP_ValveDisplay.DynMatPlate3` _asbp_valve_display_7) "EmissiveColor" (`self.DisplayGlowColor`))
      (`MaterialInstanceDynamic.SetVectorParameterValue` (`/Game/TimersClocksAndCountersPack/Blueprints/BP_ValveDisplay.DynMatPlate4` _asbp_valve_display_7) "EmissiveColor" (`self.DisplayGlowColor`))
      (`MaterialInstanceDynamic.SetVectorParameterValue` (`/Game/TimersClocksAndCountersPack/Blueprints/BP_ValveDisplay.DynMatPlate5` _asbp_valve_display_7) "EmissiveColor" (`self.DisplayGlowColor`))
      (`MaterialInstanceDynamic.SetVectorParameterValue` (`/Game/TimersClocksAndCountersPack/Blueprints/BP_ValveDisplay.DynMatPlate6` _asbp_valve_display_7) "EmissiveColor" (`self.DisplayGlowColor`))
      (`MaterialInstanceDynamic.SetVectorParameterValue` (`/Game/TimersClocksAndCountersPack/Blueprints/BP_ValveDisplay.DynMatPlate7` _asbp_valve_display_7) "EmissiveColor" (`self.DisplayGlowColor`))
      (`MaterialInstanceDynamic.SetVectorParameterValue` (`/Game/TimersClocksAndCountersPack/Blueprints/BP_ValveDisplay.DynMatPlate8` _asbp_valve_display_7) "EmissiveColor" (`self.DisplayGlowColor`))
      (`MaterialInstanceDynamic.SetVectorParameterValue` (`/Game/TimersClocksAndCountersPack/Blueprints/BP_ValveDisplay.DynMatPlateColon` _asbp_valve_display_7) "EmissiveColor" (`self.DisplayGlowColor`))
      (if (`/Game/TimersClocksAndCountersPack/Blueprints/BP_ValveDisplay.IsColon` _asbp_valve_display_7)
        (`MaterialInstanceDynamic.SetScalarParameterValue` (`/Game/TimersClocksAndCountersPack/Blueprints/BP_ValveDisplay.DynMatPlateColon` _asbp_valve_display_7) "EmissiveBrightness" (* _displayglowbrightness_4 2.0))
        (else
          (set `/Game/TimersClocksAndCountersPack/Blueprints/BP_ValveDisplay.GlowBrightness` _displayglowbrightness_4 _asbp_valve_display_7)
          (bind _displaynumber_3 (`/Game/TimersClocksAndCountersPack/Blueprints/BP_ValveDisplay.DisplayNumber` _asbp_valve_display_7))
          (`MaterialInstanceDynamic.SetScalarParameterValue` (select `int` _displaynumber_3 :`0` (`/Game/TimersClocksAndCountersPack/Blueprints/BP_ValveDisplay.DynMatPlate0` _asbp_valve_display_7) :`1` (`/Game/TimersClocksAndCountersPack/Blueprints/BP_ValveDisplay.DynMatPlate1` _asbp_valve_display_7) :`2` (`/Game/TimersClocksAndCountersPack/Blueprints/BP_ValveDisplay.DynMatPlate2` _asbp_valve_display_7) :`3` (`/Game/TimersClocksAndCountersPack/Blueprints/BP_ValveDisplay.DynMatPlate3` _asbp_valve_display_7) :`4` (`/Game/TimersClocksAndCountersPack/Blueprints/BP_ValveDisplay.DynMatPlate4` _asbp_valve_display_7) :`5` (`/Game/TimersClocksAndCountersPack/Blueprints/BP_ValveDisplay.DynMatPlate5` _asbp_valve_display_7) :`6` (`/Game/TimersClocksAndCountersPack/Blueprints/BP_ValveDisplay.DynMatPlate6` _asbp_valve_display_7) :`7` (`/Game/TimersClocksAndCountersPack/Blueprints/BP_ValveDisplay.DynMatPlate7` _asbp_valve_display_7) :`8` (`/Game/TimersClocksAndCountersPack/Blueprints/BP_ValveDisplay.DynMatPlate8` _asbp_valve_display_7) :`9` _dynmatplate9_3) "EmissiveBrightness" (* (`self.DisplayGlowBrightness`) (select `int` _displaynumber_3 :`0` 11.0 :`1` 1.0 :`2` 1.0 :`3` 1.0 :`4` 1.3 :`5` 2.0 :`6` 3.0 :`7` 5.0 :`8` 7.0 :`9` 8.0 :!type "Float (single-precision)"))))))
    (:`then_3`
      (bind _asbp_valve_display_8 (cast `/Game/TimersClocksAndCountersPack/Blueprints/BP_ValveDisplay` (`ChildActorComponent.ChildActor` (`self.MinB`))))
      (bind _dynmatvalveglass_4 (`/Game/TimersClocksAndCountersPack/Blueprints/BP_ValveDisplay.DynMatValveGlass` _asbp_valve_display_8))
      (`MaterialInstanceDynamic.SetScalarParameterValue` _dynmatvalveglass_4 "New-Old" (`self.AgeValve`))
      (`MaterialInstanceDynamic.SetScalarParameterValue` (`/Game/TimersClocksAndCountersPack/Blueprints/BP_ValveDisplay.DynMatValveEnds` _asbp_valve_display_8) "New-Old" (`self.AgeValve`))
      (`MaterialInstanceDynamic.SetScalarParameterValue` _dynmatvalveglass_4 "Roughness" (`self.RoughnessValve`))
      (`MaterialInstanceDynamic.SetScalarParameterValue` (`/Game/TimersClocksAndCountersPack/Blueprints/BP_ValveDisplay.DynMatValveEnds` _asbp_valve_display_8) "Roughness" (`self.RoughnessValve`))
      (`MaterialInstanceDynamic.SetScalarParameterValue` _dynmatvalveglass_4 "Specular" (`self.SpecularValve`))
      (`MaterialInstanceDynamic.SetScalarParameterValue` (`/Game/TimersClocksAndCountersPack/Blueprints/BP_ValveDisplay.DynMatValveEnds` _asbp_valve_display_8) "Specular" (`self.SpecularValve`))
      (`MaterialInstanceDynamic.SetScalarParameterValue` _dynmatvalveglass_4 "Metallic" (`self.MetallicValve`))
      (`MaterialInstanceDynamic.SetScalarParameterValue` (`/Game/TimersClocksAndCountersPack/Blueprints/BP_ValveDisplay.DynMatValveEnds` _asbp_valve_display_8) "Metallic" (`self.MetallicValve`))
      (`MaterialInstanceDynamic.SetScalarParameterValue` _dynmatvalveglass_4 "Normalmapstrength" (`self.NormalMapStrengthValve`))
      (`MaterialInstanceDynamic.SetScalarParameterValue` (`/Game/TimersClocksAndCountersPack/Blueprints/BP_ValveDisplay.DynMatValveEnds` _asbp_valve_display_8) "Normalmapstrength" (`self.NormalMapStrengthValve`))
      (`MaterialInstanceDynamic.SetScalarParameterValue` _dynmatvalveglass_4 "ReflactiveIndex" (`self.RefractionValveGlass`))
      (`MaterialInstanceDynamic.SetScalarParameterValue` (`/Game/TimersClocksAndCountersPack/Blueprints/BP_ValveDisplay.DynMatValveEnds` _asbp_valve_display_8) "ReflactiveIndex" (`self.RefractionValveGlass`))
      (`MaterialInstanceDynamic.SetScalarParameterValue` _dynmatvalveglass_4 "DesaturateTexture" (`self.ValveDesaturateTexture`))
      (`MaterialInstanceDynamic.SetScalarParameterValue` (`/Game/TimersClocksAndCountersPack/Blueprints/BP_ValveDisplay.DynMatValveEnds` _asbp_valve_display_8) "DesaturateTexture" (`self.ValveDesaturateTexture`))
      (bind _dynmatplate9_4 (`/Game/TimersClocksAndCountersPack/Blueprints/BP_ValveDisplay.DynMatPlate9` _asbp_valve_display_8))
      (`MaterialInstanceDynamic.SetVectorParameterValue` _dynmatplate9_4 "EmissiveColor" (`self.DisplayGlowColor`))
      (`MaterialInstanceDynamic.SetVectorParameterValue` (`/Game/TimersClocksAndCountersPack/Blueprints/BP_ValveDisplay.DynMatPlate0` _asbp_valve_display_8) "EmissiveColor" (`self.DisplayGlowColor`))
      (`MaterialInstanceDynamic.SetVectorParameterValue` (`/Game/TimersClocksAndCountersPack/Blueprints/BP_ValveDisplay.DynMatPlate1` _asbp_valve_display_8) "EmissiveColor" (`self.DisplayGlowColor`))
      (`MaterialInstanceDynamic.SetVectorParameterValue` (`/Game/TimersClocksAndCountersPack/Blueprints/BP_ValveDisplay.DynMatPlate2` _asbp_valve_display_8) "EmissiveColor" (`self.DisplayGlowColor`))
      (`MaterialInstanceDynamic.SetVectorParameterValue` (`/Game/TimersClocksAndCountersPack/Blueprints/BP_ValveDisplay.DynMatPlate3` _asbp_valve_display_8) "EmissiveColor" (`self.DisplayGlowColor`))
      (`MaterialInstanceDynamic.SetVectorParameterValue` (`/Game/TimersClocksAndCountersPack/Blueprints/BP_ValveDisplay.DynMatPlate4` _asbp_valve_display_8) "EmissiveColor" (`self.DisplayGlowColor`))
      (`MaterialInstanceDynamic.SetVectorParameterValue` (`/Game/TimersClocksAndCountersPack/Blueprints/BP_ValveDisplay.DynMatPlate5` _asbp_valve_display_8) "EmissiveColor" (`self.DisplayGlowColor`))
      (`MaterialInstanceDynamic.SetVectorParameterValue` (`/Game/TimersClocksAndCountersPack/Blueprints/BP_ValveDisplay.DynMatPlate6` _asbp_valve_display_8) "EmissiveColor" (`self.DisplayGlowColor`))
      (`MaterialInstanceDynamic.SetVectorParameterValue` (`/Game/TimersClocksAndCountersPack/Blueprints/BP_ValveDisplay.DynMatPlate7` _asbp_valve_display_8) "EmissiveColor" (`self.DisplayGlowColor`))
      (`MaterialInstanceDynamic.SetVectorParameterValue` (`/Game/TimersClocksAndCountersPack/Blueprints/BP_ValveDisplay.DynMatPlate8` _asbp_valve_display_8) "EmissiveColor" (`self.DisplayGlowColor`))
      (`MaterialInstanceDynamic.SetVectorParameterValue` (`/Game/TimersClocksAndCountersPack/Blueprints/BP_ValveDisplay.DynMatPlateColon` _asbp_valve_display_8) "EmissiveColor" (`self.DisplayGlowColor`))
      (if (`/Game/TimersClocksAndCountersPack/Blueprints/BP_ValveDisplay.IsColon` _asbp_valve_display_8)
        (`MaterialInstanceDynamic.SetScalarParameterValue` (`/Game/TimersClocksAndCountersPack/Blueprints/BP_ValveDisplay.DynMatPlateColon` _asbp_valve_display_8) "EmissiveBrightness" (* _displayglowbrightness_5 2.0))
        (else
          (set `/Game/TimersClocksAndCountersPack/Blueprints/BP_ValveDisplay.GlowBrightness` _displayglowbrightness_5 _asbp_valve_display_8)
          (bind _displaynumber_4 (`/Game/TimersClocksAndCountersPack/Blueprints/BP_ValveDisplay.DisplayNumber` _asbp_valve_display_8))
          (`MaterialInstanceDynamic.SetScalarParameterValue` (select `int` _displaynumber_4 :`0` (`/Game/TimersClocksAndCountersPack/Blueprints/BP_ValveDisplay.DynMatPlate0` _asbp_valve_display_8) :`1` (`/Game/TimersClocksAndCountersPack/Blueprints/BP_ValveDisplay.DynMatPlate1` _asbp_valve_display_8) :`2` (`/Game/TimersClocksAndCountersPack/Blueprints/BP_ValveDisplay.DynMatPlate2` _asbp_valve_display_8) :`3` (`/Game/TimersClocksAndCountersPack/Blueprints/BP_ValveDisplay.DynMatPlate3` _asbp_valve_display_8) :`4` (`/Game/TimersClocksAndCountersPack/Blueprints/BP_ValveDisplay.DynMatPlate4` _asbp_valve_display_8) :`5` (`/Game/TimersClocksAndCountersPack/Blueprints/BP_ValveDisplay.DynMatPlate5` _asbp_valve_display_8) :`6` (`/Game/TimersClocksAndCountersPack/Blueprints/BP_ValveDisplay.DynMatPlate6` _asbp_valve_display_8) :`7` (`/Game/TimersClocksAndCountersPack/Blueprints/BP_ValveDisplay.DynMatPlate7` _asbp_valve_display_8) :`8` (`/Game/TimersClocksAndCountersPack/Blueprints/BP_ValveDisplay.DynMatPlate8` _asbp_valve_display_8) :`9` _dynmatplate9_4) "EmissiveBrightness" (* (`self.DisplayGlowBrightness`) (select `int` _displaynumber_4 :`0` 11.0 :`1` 1.0 :`2` 1.0 :`3` 1.0 :`4` 1.3 :`5` 2.0 :`6` 3.0 :`7` 5.0 :`8` 7.0 :`9` 8.0 :!type "Float (single-precision)"))))))
    (:`then_4`
      (bind _asbp_valve_display_9 (cast `/Game/TimersClocksAndCountersPack/Blueprints/BP_ValveDisplay` (`ChildActorComponent.ChildActor` (`self.Colon`))))
      (bind _dynmatvalveglass_5 (`/Game/TimersClocksAndCountersPack/Blueprints/BP_ValveDisplay.DynMatValveGlass` _asbp_valve_display_9))
      (`MaterialInstanceDynamic.SetScalarParameterValue` _dynmatvalveglass_5 "New-Old" (`self.AgeValve`))
      (`MaterialInstanceDynamic.SetScalarParameterValue` (`/Game/TimersClocksAndCountersPack/Blueprints/BP_ValveDisplay.DynMatValveEnds` _asbp_valve_display_9) "New-Old" (`self.AgeValve`))
      (`MaterialInstanceDynamic.SetScalarParameterValue` _dynmatvalveglass_5 "Roughness" (`self.RoughnessValve`))
      (`MaterialInstanceDynamic.SetScalarParameterValue` (`/Game/TimersClocksAndCountersPack/Blueprints/BP_ValveDisplay.DynMatValveEnds` _asbp_valve_display_9) "Roughness" (`self.RoughnessValve`))
      (`MaterialInstanceDynamic.SetScalarParameterValue` _dynmatvalveglass_5 "Specular" (`self.SpecularValve`))
      (`MaterialInstanceDynamic.SetScalarParameterValue` (`/Game/TimersClocksAndCountersPack/Blueprints/BP_ValveDisplay.DynMatValveEnds` _asbp_valve_display_9) "Specular" (`self.SpecularValve`))
      (`MaterialInstanceDynamic.SetScalarParameterValue` _dynmatvalveglass_5 "Metallic" (`self.MetallicValve`))
      (`MaterialInstanceDynamic.SetScalarParameterValue` (`/Game/TimersClocksAndCountersPack/Blueprints/BP_ValveDisplay.DynMatValveEnds` _asbp_valve_display_9) "Metallic" (`self.MetallicValve`))
      (`MaterialInstanceDynamic.SetScalarParameterValue` _dynmatvalveglass_5 "Normalmapstrength" (`self.NormalMapStrengthValve`))
      (`MaterialInstanceDynamic.SetScalarParameterValue` (`/Game/TimersClocksAndCountersPack/Blueprints/BP_ValveDisplay.DynMatValveEnds` _asbp_valve_display_9) "Normalmapstrength" (`self.NormalMapStrengthValve`))
      (`MaterialInstanceDynamic.SetScalarParameterValue` _dynmatvalveglass_5 "ReflactiveIndex" (`self.RefractionValveGlass`))
      (`MaterialInstanceDynamic.SetScalarParameterValue` (`/Game/TimersClocksAndCountersPack/Blueprints/BP_ValveDisplay.DynMatValveEnds` _asbp_valve_display_9) "ReflactiveIndex" (`self.RefractionValveGlass`))
      (`MaterialInstanceDynamic.SetScalarParameterValue` _dynmatvalveglass_5 "DesaturateTexture" (`self.ValveDesaturateTexture`))
      (`MaterialInstanceDynamic.SetScalarParameterValue` (`/Game/TimersClocksAndCountersPack/Blueprints/BP_ValveDisplay.DynMatValveEnds` _asbp_valve_display_9) "DesaturateTexture" (`self.ValveDesaturateTexture`))
      (bind _dynmatplate9_5 (`/Game/TimersClocksAndCountersPack/Blueprints/BP_ValveDisplay.DynMatPlate9` _asbp_valve_display_9))
      (`MaterialInstanceDynamic.SetVectorParameterValue` _dynmatplate9_5 "EmissiveColor" (`self.DisplayGlowColor`))
      (`MaterialInstanceDynamic.SetVectorParameterValue` (`/Game/TimersClocksAndCountersPack/Blueprints/BP_ValveDisplay.DynMatPlate0` _asbp_valve_display_9) "EmissiveColor" (`self.DisplayGlowColor`))
      (`MaterialInstanceDynamic.SetVectorParameterValue` (`/Game/TimersClocksAndCountersPack/Blueprints/BP_ValveDisplay.DynMatPlate1` _asbp_valve_display_9) "EmissiveColor" (`self.DisplayGlowColor`))
      (`MaterialInstanceDynamic.SetVectorParameterValue` (`/Game/TimersClocksAndCountersPack/Blueprints/BP_ValveDisplay.DynMatPlate2` _asbp_valve_display_9) "EmissiveColor" (`self.DisplayGlowColor`))
      (`MaterialInstanceDynamic.SetVectorParameterValue` (`/Game/TimersClocksAndCountersPack/Blueprints/BP_ValveDisplay.DynMatPlate3` _asbp_valve_display_9) "EmissiveColor" (`self.DisplayGlowColor`))
      (`MaterialInstanceDynamic.SetVectorParameterValue` (`/Game/TimersClocksAndCountersPack/Blueprints/BP_ValveDisplay.DynMatPlate4` _asbp_valve_display_9) "EmissiveColor" (`self.DisplayGlowColor`))
      (`MaterialInstanceDynamic.SetVectorParameterValue` (`/Game/TimersClocksAndCountersPack/Blueprints/BP_ValveDisplay.DynMatPlate5` _asbp_valve_display_9) "EmissiveColor" (`self.DisplayGlowColor`))
      (`MaterialInstanceDynamic.SetVectorParameterValue` (`/Game/TimersClocksAndCountersPack/Blueprints/BP_ValveDisplay.DynMatPlate6` _asbp_valve_display_9) "EmissiveColor" (`self.DisplayGlowColor`))
      (`MaterialInstanceDynamic.SetVectorParameterValue` (`/Game/TimersClocksAndCountersPack/Blueprints/BP_ValveDisplay.DynMatPlate7` _asbp_valve_display_9) "EmissiveColor" (`self.DisplayGlowColor`))
      (`MaterialInstanceDynamic.SetVectorParameterValue` (`/Game/TimersClocksAndCountersPack/Blueprints/BP_ValveDisplay.DynMatPlate8` _asbp_valve_display_9) "EmissiveColor" (`self.DisplayGlowColor`))
      (`MaterialInstanceDynamic.SetVectorParameterValue` (`/Game/TimersClocksAndCountersPack/Blueprints/BP_ValveDisplay.DynMatPlateColon` _asbp_valve_display_9) "EmissiveColor" (`self.DisplayGlowColor`))
      (if (`/Game/TimersClocksAndCountersPack/Blueprints/BP_ValveDisplay.IsColon` _asbp_valve_display_9)
        (`MaterialInstanceDynamic.SetScalarParameterValue` (`/Game/TimersClocksAndCountersPack/Blueprints/BP_ValveDisplay.DynMatPlateColon` _asbp_valve_display_9) "EmissiveBrightness" (* _displayglowbrightness 2.0))
        (else
          (set `/Game/TimersClocksAndCountersPack/Blueprints/BP_ValveDisplay.GlowBrightness` _displayglowbrightness _asbp_valve_display_9)
          (bind _displaynumber_5 (`/Game/TimersClocksAndCountersPack/Blueprints/BP_ValveDisplay.DisplayNumber` _asbp_valve_display_9))
          (`MaterialInstanceDynamic.SetScalarParameterValue` (select `int` _displaynumber_5 :`0` (`/Game/TimersClocksAndCountersPack/Blueprints/BP_ValveDisplay.DynMatPlate0` _asbp_valve_display_9) :`1` _dynmatplate9_5 :`2` (`/Game/TimersClocksAndCountersPack/Blueprints/BP_ValveDisplay.DynMatPlate2` _asbp_valve_display_9) :`3` (`/Game/TimersClocksAndCountersPack/Blueprints/BP_ValveDisplay.DynMatPlate3` _asbp_valve_display_9) :`4` (`/Game/TimersClocksAndCountersPack/Blueprints/BP_ValveDisplay.DynMatPlate4` _asbp_valve_display_9) :`5` (`/Game/TimersClocksAndCountersPack/Blueprints/BP_ValveDisplay.DynMatPlate5` _asbp_valve_display_9) :`6` (`/Game/TimersClocksAndCountersPack/Blueprints/BP_ValveDisplay.DynMatPlate6` _asbp_valve_display_9) :`7` (`/Game/TimersClocksAndCountersPack/Blueprints/BP_ValveDisplay.DynMatPlate7` _asbp_valve_display_9) :`8` (`/Game/TimersClocksAndCountersPack/Blueprints/BP_ValveDisplay.DynMatPlate8` _asbp_valve_display_9) :`9` _dynmatplate9_5) "EmissiveBrightness" (* (`self.DisplayGlowBrightness`) (select `int` _displaynumber_5 :`0` 11.0 :`1` 1.0 :`2` 1.0 :`3` 1.0 :`4` 1.3 :`5` 2.0 :`6` 3.0 :`7` 5.0 :`8` 7.0 :`9` 8.0 :!type "Float (single-precision)"))))))))