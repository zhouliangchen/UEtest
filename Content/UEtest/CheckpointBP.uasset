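; Clock-themed checkpoint that, on interaction, becomes active and saves the game through UEtestGameModeBase on the authority.
; Activation saves the time, turns on particles, sets TickActive false and drives clock material parameters for second-hand flash and hit timing.
; The OnRep of the cached time mirrors activation and restores the saved time; OnActorLoaded does the same for active checkpoints, without the hit effect.
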(event `MGameplayInterface.Interact`
  (params (InstigatorPawn :type "Pawn Object Reference"))
  (`/Engine/EditorBlueprintResources/ActorMacros.Switch Has Authority`
    (:`Authority`
      (set `self.bActive` true)
      (`self.Save Time`)
      (bind _asuetest_game_mode_base (cast `UEtestGameModeBase` (`GameplayStatics.GetGameMode`)))
      (`UEtestGameModeBase.WriteSaveGame` _asuetest_game_mode_base)
      (`KismetSystemLibrary.PrintString` "Game Saved")
      (`self.UpdateCheckPoint`)
      (`MeshComponent.SetScalarParameterValueOnMaterials` (`self.SM_AnalogueClockHousing01`) "TimeOnHit" (`self.GetGameTimeSinceCreation`)))))

(event `self.UpdateCheckPoint`
  (`parent.UpdateCheckPoint`)
  (if (`self.bActive`)
    (`ActorComponent.Activate` (`self.ParticleSystem`) false)
    (set `self.bTickActive` false)
    (`MeshComponent.SetScalarParameterValueOnMaterials` (`self.SM_AnalogueClockSecondHand01`) "bFlash" 2.0)))

(event `MGameplayInterface.OnActorLoaded`
  (if (`self.bActive`)
    (`self.UpdateCheckPoint`)
    (`self.Load Time` (`self.CustomTimeCacheHour`) (`self.CustomTimeCacheMinute`) (`self.CustomTimeCacheSecond`))))

(event `self.OnRep_CustomTimeCache`
  (bind _customtimecache (`self.CustomTimeCache`))
  (bind (_year _month _day _hour _minute _second) (`KismetMathLibrary.BreakDateTime` _customtimecache))
  (set `self.bActive` true)
  (`self.UpdateCheckPoint`)
  (`self.Load Time` (`KismetMathLibrary.GetHour12` _customtimecache) _minute _second)
  (`MeshComponent.SetScalarParameterValueOnMaterials` (`self.SM_AnalogueClockHousing01`) "TimeOnHit" (`self.GetGameTimeSinceCreation`)))

(fn `UserConstructionScript`)