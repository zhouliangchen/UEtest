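; Player controller Blueprint that sets up the main HUD and provides a save-game hotkey.
; The HUD is created for local controllers only: from BeginPlay with authority, or from the player-state replicated event, which also switches input to game-only.
; Pressing K with authority calls WriteSaveGame on UEtestGameModeBase and prints a confirmation, so only the host can save this way.
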(event `self.ReceiveBeginPlay`
  (`/Engine/EditorBlueprintResources/ActorMacros.Switch Has Authority`
    (:`Authority`
      (if (`self.IsLocalController`) :!label _label
        (bind _returnvalue (`|CreateWidget` "/Game/UEtest/UI/MainHUD.MainHUD_C"))
        (`UserWidget.AddToViewport` _returnvalue 0)
        (`WidgetBlueprintLibrary.SetInputMode_GameOnly` self)))))

(event `self.OnPlayerStateReplicatedBP`
  (params (NewPlayerState :type "PlayerState Object Reference"))
  (goto _label))

(event `Key|K`
  (params (Key :type "Key Structure"))
  (:`Pressed`
    (`/Engine/EditorBlueprintResources/ActorMacros.Switch Has Authority`
      (:`Authority`
        (bind _asuetest_game_mode_base (cast `UEtestGameModeBase` (`GameplayStatics.GetGameMode`)))
        (`UEtestGameModeBase.WriteSaveGame` _asuetest_game_mode_base)
        (`KismetSystemLibrary.PrintString` "Game Saved")))))

(fn `UserConstructionScript`)